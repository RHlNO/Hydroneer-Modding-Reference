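; Buildable pipe filter that raises the quality of water passing through it at a small cost in pressure.
; Each pass wears durability, faster for dirtier water, and updates a text readout before the parent's water swap forwards the flow.
; Signals relay between its two boxes, but worn-out filters send them as off and stop passing water.
; Activating it while carrying a tool bag restores full durability.
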(event `self.WaterIn`
  (params (Box :type String) (WaterQuality :type Integer) (WaterPressure :type "Float (single-precision)"))
  (if (>= (`self.Durability`) 25.0)
    (bind _output_get (set `self.Durability` (`KismetMathLibrary.FClamp` (- (`self.Durability`) (/ (`KismetMathLibrary.Conv_IntToDouble` (- 10 WaterQuality)) 400.0)) 0.0 100.0)))
    (`TextRenderComponent.K2_SetText` (`self.TextRender_0`) (`KismetTextLibrary.Conv_DoubleToText` _output_get "HalfToEven"))
    (`parent.WaterSwap` Box (+ WaterQuality 2) (- WaterPressure 1.0))))

(event `self.SignalIn`
  (params (Box :type String) (Active :type Boolean))
  (bind _signaloff (`self.SignalOff`))
  (set `self.SignalOff` Active)
  (if (not (> (`self.Durability`) 25.0))
    (set `self.SignalOff` false))
  (switch `string` Box
    (:`Box1`
      (`self.SendSignal` (`self.Box2`) _signaloff))
    (:`Box2`
      (`self.SendSignal` (`self.Box1`) _signaloff))))

(event `/Game/WorldObjects/Items/BP_ParentItem.OverrideMouseActivated`
  (params (Component :type "ActorComponent Object Reference"))
  (bind _asbp_game_controller (cast `/Game/BP_GameController` (`GameplayStatics.GetPlayerController` 0)))
  (bind _asbp_tool_bag (cast `/Game/WorldObjects/Items/ToolItems/BP_ToolBag` (`/Game/BP_GameController.CarryingItem` _asbp_game_controller)))
  (set `self.Durability` 100.0)
  (`/Game/WorldObjects/Items/ToolItems/BP_ToolBag.DoRepair` _asbp_tool_bag))

(fn `UserConstructionScript`
  (`parent.UserConstructionScript`))