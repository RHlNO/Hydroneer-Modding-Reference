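; BP_PipeDelay is a buildable pipe item that delays signals passing between its two boxes, while handing water input to parent logic.
; Incoming signals queue in a History buffer; once it exceeds Delay, the oldest goes out the opposite box.
; Each forwarded signal restarts a short timer that clears the buffer.
; Mouse activation cycles Delay with wraparound, clears the buffer and displays Delay in tenths.
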(event `CustomEvent_0`
  (set `self.History` (`|MakeArray`)))

(event `self.SignalIn`
  (params (Box :type String) (Active :type Boolean))
  (bind _history (`self.History`))
  (bind _history_2 (`self.History`))
  (bind _signaltemp (`self.SignalTemp`))
  (`KismetArrayLibrary.Array_Add` _history Active)
  (if (> (`KismetArrayLibrary.Array_Length` _history) (`self.Delay`))
    (set `self.SignalTemp` (`|GetArrayItem` _history_2))
    (`KismetArrayLibrary.Array_Remove` _history_2)
    (`KismetSystemLibrary.K2_SetTimerDelegate` (delegate `CustomEvent_0`) 0.15)
    (switch `string` Box
      (:`Box1`
        (`self.SendSignal` (`self.Box2`) _signaltemp))
      (:`Box2`
        (`self.SendSignal` (`self.Box1`) _signaltemp)))))

(event `self.WaterIn`
  (params (Box :type String) (WaterQuality :type Integer) (WaterPressure :type "Float (single-precision)"))
  (`parent.WaterSwap` Box WaterQuality WaterPressure))

(event `/Game/WorldObjects/Items/BP_ParentItem.OverrideMouseActivated`
  (params (Component :type "ActorComponent Object Reference"))
  (bind _output_get (set `self.Delay` (+ (`self.Delay`) 1)))
  (if (> _output_get 10)
    (set `self.Delay` 0))
  (set `self.History` (`|MakeArray`))
  (`TextRenderComponent.K2_SetText` (`self.TextRender5`) (`KismetTextLibrary.Conv_DoubleToText` (/ (`KismetMathLibrary.Conv_IntToDouble` (`self.Delay`)) 10.0) "HalfToEven"))
  (bind _asbp_game_controller (cast `/Game/BP_GameController` (`GameplayStatics.GetPlayerController` 0)))
  (`/Game/BP_GameController.ReturnNoActivation` _asbp_game_controller (`ActorComponent.GetOwner` Component)))

(fn `UserConstructionScript`
  (`parent.UserConstructionScript`)
  (`TextRenderComponent.K2_SetText` (`self.TextRender5`) (`KismetTextLibrary.Conv_IntToText` (`self.Delay`))))