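; Pipe valve build item that gates water and relays signals between its two boxes, with Auto, Off and On modes.
; Mouse activation cycles the mode, updating the text label and animating the valve mesh with a turn sound for Off and On.
; Incoming signals recompute the blocked state (Auto opens only on an active signal) and pass to the opposite box, forced false when blocked.
; Water reaches the parent's swap logic only while unblocked.
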(event `self.SignalIn`
  (params (Box :type String) (Active :type Boolean))
  (bind _signal (`self.Signal`))
  (set `self.Signal` Active)
  (bind _output_get (set `self.Blocked?` (not (or (== (`self.Toggle`) 2) (and (== (`self.Toggle`) 0) Active)))))
  (if _output_get
    (set `self.Signal` false))
  (switch `string` Box
    (:`Box1`
      (`self.SendSignal` (`self.Box2`) _signal))
    (:`Box2`
      (`self.SendSignal` (`self.Box1`) _signal))))

(event `self.WaterIn`
  (params (Box :type String) (WaterQuality :type Integer) (WaterPressure :type "Float (single-precision)"))
  (if (not (`self.Blocked?`))
    (`parent.WaterSwap` Box WaterQuality WaterPressure)))

(event `/Game/WorldObjects/Items/BP_ParentItem.OverrideMouseActivated`
  (params (Component :type "ActorComponent Object Reference"))
  (switch `int` (`self.Toggle`)
    (:`0`
      (set `self.Toggle` 1))
    (:`1`
      (set `self.Toggle` 2))
    (:`2`
      (set `self.Toggle` 0)))
  (`self.UpdateState` true))

(event `UpdateState`
  (params (`Sound?` :type Boolean))
  (bind _staticmesh1 (`self.StaticMesh1`))
  (bind _textrender_0 (`self.TextRender_0`))
  (switch `int` (`self.Toggle`)
    (:`0`
      (`TextRenderComponent.K2_SetText` _textrender_0 (`KismetTextLibrary.Conv_StringToText` "Auto")))
    (:`1`
      (`TextRenderComponent.K2_SetText` _textrender_0 (`KismetTextLibrary.Conv_StringToText` "Off"))
      (if `Sound?`
        (`GameplayStatics.SpawnSoundAttached` "/Game/Sound/Construction/Valve_Turn.Valve_Turn" _staticmesh1 "None" (0.0 0.0 0.0) (struct) "KeepRelativeOffset" true 1.0 1.0 0.0 "/Game/Sound/EnvLoops/SA_SmallEnv.SA_SmallEnv" null)
        (bind (_direction _newtrack_0) (`Timeline|Timeline_1` :!label _label)
          (:`Update`
            (`SceneComponent.K2_SetRelativeRotation` _staticmesh1 (`KismetMathLibrary.MakeRotator` 0.0 0.0 _newtrack_0) false false)))
        (else
          (goto _label))))
    (:`2`
      (`TextRenderComponent.K2_SetText` _textrender_0 (`KismetTextLibrary.Conv_StringToText` "On"))
      (if `Sound?`
        (`GameplayStatics.SpawnSoundAttached` "/Game/Sound/Construction/Valve_Turn.Valve_Turn" _staticmesh1 "None" (0.0 0.0 0.0) (struct) "KeepRelativeOffset" true 1.0 1.0 0.0 "/Game/Sound/EnvLoops/SA_SmallEnv.SA_SmallEnv" null)
        (goto _label :!via `ReverseFromEnd`)
        (else
          (goto _label :!via `ReverseFromEnd`))))))

(fn `UserConstructionScript`
  (`parent.UserConstructionScript`)
  (`KismetArrayLibrary.Array_Add` (`self.ExtraMeshes`) (`self.StaticMesh1`)))