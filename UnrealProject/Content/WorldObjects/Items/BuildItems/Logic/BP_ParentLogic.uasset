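; Base Blueprint for placeable logic build items that pass water and electrical signals between neighbours through six box ports.
; Short line traces at a port find the adjacent item to call WaterIn or SignalIn, an empty hook here; unconnected, uncorked water outlets spawn projectiles.
; Water loses pressure per hop, with timers and a signal counter throttling propagation.
; Pipe and cable materials show state, while timelines slide indicators to show flow.
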(event `CustomEvent`
  (set `self.WaterIn?` false))

(event `WaterSwap`
  (params (NewParam :type String) (NewParam2 :type Integer) (NewParam3 :type "Float (double-precision)"))
  (if (not (`self.WaterIn?`))
    (set `self.WaterIn?` true)
    (`KismetSystemLibrary.K2_SetTimerDelegate` (delegate `CustomEvent`) 0.75)
    (switch `string` NewParam
      (:`Box1`
        (`self.SendWater` (`self.Box2`) NewParam2 NewParam3))
      (:`Box2`
        (`self.SendWater` (`self.Box1`) NewParam2 NewParam3))
      (:`Box3`
        (`self.SendWater` (`self.Box4`) NewParam2 NewParam3))
      (:`Box4`
        (`self.SendWater` (`self.Box3`) NewParam2 NewParam3))
      (:`Box5`
        (`self.SendWater` (`self.Box6`)))
      (:`Box6`
        (`self.SendWater` (`self.Box5`))))))

(event `IndicatorMove`
  (params (NewParam :type String))
  (bind _indicator1 (`self.Indicator1`))
  (bind _indicator6 (`self.Indicator6`))
  (bind _indicator2 (`self.Indicator2`))
  (bind _indicator3 (`self.Indicator3`))
  (bind _indicator5 (`self.Indicator5`))
  (bind _indicator4 (`self.Indicator4`))
  (switch `string` NewParam
    (:`Box1`
      (bind (_direction _newtrack_0) (`Timeline|Timeline_0` :!via `PlayFromStart`)
        (:`Update`
          (`SceneComponent.K2_SetRelativeLocation` _indicator1 (`KismetMathLibrary.MakeVector` 0.0 _newtrack_0 21.0) false false)
          (`SceneComponent.K2_SetRelativeLocation` _indicator6 (0.0 0.0 -21.0) false false)
          (bind _returnvalue (+ _newtrack_0 33.333))
          (`SceneComponent.K2_SetRelativeLocation` _indicator2 (`KismetMathLibrary.MakeVector` 0.0 _returnvalue 21.0) false false)
          (`SceneComponent.K2_SetRelativeLocation` _indicator5 (`KismetMathLibrary.MakeVector` 0.0 _returnvalue -21.0) false false)
          (bind _returnvalue_2 (+ _returnvalue 33.333))
          (`SceneComponent.K2_SetRelativeLocation` _indicator3 (`KismetMathLibrary.MakeVector` 0.0 _returnvalue_2 21.0) false false)
          (`SceneComponent.K2_SetRelativeLocation` _indicator4 (`KismetMathLibrary.MakeVector` 0.0 _returnvalue_2 21.0) false false))))
    (:`Box2`
      (bind (_direction_2 _newtrack_0_2) (`Timeline|MoveCylinders` :!via `PlayFromStart`)
        (:`Update`
          (`SceneComponent.K2_SetRelativeLocation` _indicator1 (`KismetMathLibrary.MakeVector` 0.0 _newtrack_0_2 21.0) false false)
          (`SceneComponent.K2_SetRelativeLocation` _indicator6 (`KismetMathLibrary.MakeVector` 0.0 _newtrack_0_2 -21.0) false false)
          (bind _returnvalue_3 (- _newtrack_0_2 33.333))
          (`SceneComponent.K2_SetRelativeLocation` _indicator2 (`KismetMathLibrary.MakeVector` 0.0 _returnvalue_3 21.0) false false)
          (`SceneComponent.K2_SetRelativeLocation` _indicator5 (`KismetMathLibrary.MakeVector` 0.0 _returnvalue_3 -21.0) false false)
          (bind _returnvalue_4 (- _returnvalue_3 33.333))
          (`SceneComponent.K2_SetRelativeLocation` _indicator3 (`KismetMathLibrary.MakeVector` 0.0 _returnvalue_4 21.0) false false)
          (`SceneComponent.K2_SetRelativeLocation` _indicator4 (`KismetMathLibrary.MakeVector` 0.0 _returnvalue_4 -21.0) false false))))))

(event `WaterBlock`
  (set `self.WaterIn?` false))

(event `self.WaterIn`
  (params (Box :type String) (WaterQuality :type Integer) (WaterPressure :type "Float (single-precision)"))
  (if (and (`self.PlacedDown?`) (not (`self.WaterIn?`)))
    (set `self.WaterIn?` true)
    (`KismetSystemLibrary.K2_SetTimerDelegate` (delegate `WaterBlock`) 0.75)
    (`self.SendWater` (`self.Box3`) WaterQuality WaterPressure)))

(event `/Game/WorldObjects/Items/BP_ParentItem.OverrideMouseActivated`
  (params (Component :type "ActorComponent Object Reference"))
  (bind _asbp_game_controller (cast `/Game/BP_GameController` (`GameplayStatics.GetPlayerController` 0)))
  (`/Game/BP_GameController.ReturnNoActivation` _asbp_game_controller (`ActorComponent.GetOwner` Component)))

(fn `CountInputs`
  (set `self.TotalIn` 0)
  (set `self.TotalPlus` 0)
  (for _array_element (`self.Inputs`)
    (if _array_element
      (set `self.TotalIn` (+ (`self.TotalIn`) 1))))
  (for _array_element_2 (`self.Flow`)
    (if _array_element_2
      (set `self.TotalPlus` (+ (`self.TotalPlus`) 1)))))

(fn `ElectricBlack`
  (`PrimitiveComponent.SetMaterial` (`self.ElectricCable`) 0 "/Game/Materials/M_Black.M_Black")
  (`PrimitiveComponent.SetMaterial` (`self.ElectricCable2`) 0 "/Game/Materials/M_Black.M_Black")
  (`PrimitiveComponent.SetMaterial` (`self.ElectricCable3`) 0 "/Game/Materials/M_Black.M_Black")
  (`PrimitiveComponent.SetMaterial` (`self.ElectricCable4`) 0 "/Game/Materials/M_Black.M_Black")
  (set `self.LastPulse` false))

(fn `ElectricColour`
  (params (Colour :type "Material Object Reference"))
  (`PrimitiveComponent.SetMaterial` (`self.ElectricCable`) 0 Colour)
  (`PrimitiveComponent.SetMaterial` (`self.ElectricCable2`) 0 Colour)
  (`PrimitiveComponent.SetMaterial` (`self.ElectricCable3`) 0 Colour)
  (`PrimitiveComponent.SetMaterial` (`self.ElectricCable4`) 0 Colour))

(fn `GenerateSignal`
  (bind _box2 (`self.Box2`))
  (bind (_returnvalue_x _returnvalue_y _returnvalue_z) (`KismetMathLibrary.BreakVector` (`SceneComponent.K2_GetComponentLocation` _box2)))
  (if (`self.PlacedDown?`)
    (bind _outhit (`KismetSystemLibrary.LineTraceSingle` (`SceneComponent.K2_GetComponentLocation` _box2) (`KismetMathLibrary.MakeVector` _returnvalue_x _returnvalue_y (+ _returnvalue_z 1.0)) "TraceTypeQuery1" true))
    (bind (_bblockinghit _binitialoverlap _time _distance _location _impactpoint _normal _impactnormal _physmat _hitactor _hitcomponent) (`GameplayStatics.BreakHitResult` _outhit))
    (bind _asbp_parent_logic (cast `/Game/WorldObjects/Items/BuildItems/Logic/BP_ParentLogic` _hitactor))
    (`self.SignalIn` _asbp_parent_logic (`KismetSystemLibrary.GetObjectName` _hitcomponent) true)))

(fn `Off0`
  (`KismetArrayLibrary.Array_Set` (`self.Inputs`))
  (`self.CountInputs`)
  (`KismetArrayLibrary.Array_Set` (`self.Flow`)))

(fn `Off1`
  (`KismetArrayLibrary.Array_Set` (`self.Inputs`) 1)
  (`self.CountInputs`)
  (`KismetArrayLibrary.Array_Set` (`self.Flow`) 1))

(fn `Off2`
  (`KismetArrayLibrary.Array_Set` (`self.Inputs`) 2)
  (`self.CountInputs`)
  (`KismetArrayLibrary.Array_Set` (`self.Flow`) 2))

(fn `Off3`
  (`KismetArrayLibrary.Array_Set` (`self.Inputs`) 3)
  (`self.CountInputs`)
  (`KismetArrayLibrary.Array_Set` (`self.Flow`) 3))

(fn `Off4`
  (`KismetArrayLibrary.Array_Set` (`self.Inputs`) 4)
  (`self.CountInputs`)
  (`KismetArrayLibrary.Array_Set` (`self.Flow`) 4))

(fn `Off5`
  (`KismetArrayLibrary.Array_Set` (`self.Inputs`) 5)
  (`self.CountInputs`)
  (`KismetArrayLibrary.Array_Set` (`self.Flow`) 5))

(fn `SendSignal`
  (params (Box :type "BoxComponent Object Reference") (Active :type Boolean))
  (locals (NewLocalVar_0 :type "Box Structure" :default (struct :`Min` (1.0 1.0 1.0) :`Max` (5.0 5.0 5.0))) (NewLocalVar_1 :type "Array of EObjectTypeQuery Enum"))
  (bind (_returnvalue_x _returnvalue_y _returnvalue_z) (`KismetMathLibrary.BreakVector` (`SceneComponent.K2_GetComponentLocation` Box)))
  (bind (_returnvalue_x_2 _returnvalue_y_2 _returnvalue_z_2) (`KismetMathLibrary.BreakVector` (`SceneComponent.K2_GetComponentLocation` Box)))
  (bind _thispulse (`self.ThisPulse`))
  (if (`self.SignalReset`)
    (`KismetSystemLibrary.K2_SetTimer` null "UnsetSignal" 0.05)
    (set `self.SignalReset` false))
  (if (and (`self.PlacedDown?`) (< (`self.SignalCount`) 7))
    (set `self.ThisPulse` Active)
    (bind _outhit (`KismetSystemLibrary.LineTraceSingle` :`Start` (`KismetMathLibrary.MakeVector` (- _returnvalue_x_2 2.0) (- _returnvalue_y_2 2.0) (- _returnvalue_z_2 2.0)) :`End` (`KismetMathLibrary.MakeVector` (+ _returnvalue_x 2.0) (+ _returnvalue_y 2.0) (+ _returnvalue_z 2.0)) :`TraceChannel` "TraceTypeQuery1" :`bTraceComplex` true :`DrawDebugType` "Persistent" :`TraceColor` (struct :`G` 0.059102 :`B` 1.0 :`A` 1.0)))
    (set `self.SignalCount` (+ (`self.SignalCount`) 1))
    (if (or (`KismetStringLibrary.EqualEqual_StrStr` (`KismetSystemLibrary.GetObjectName` (`PrimitiveComponent.GetMaterial` (`self.ElectricCable`) 0)) "M_Black") (xor (`self.LastPulse`) _thispulse))
      (if _thispulse
        (`self.ElectricColour` "/Game/Materials/M_Green.M_Green")
        (else
          (`self.ElectricColour` "/Game/Materials/M_Red.M_Red"))))
    (`KismetSystemLibrary.K2_SetTimer` null "ResetElectric" 0.15)
    (set `self.LastPulse` _thispulse)
    (bind (_bblockinghit _binitialoverlap _time _distance _location _impactpoint _normal _impactnormal _physmat _hitactor _hitcomponent) (`GameplayStatics.BreakHitResult` _outhit))
    (bind _asbp_parent_logic (cast `/Game/WorldObjects/Items/BuildItems/Logic/BP_ParentLogic` _hitactor)
      (:`then`
        (`self.SignalIn` _asbp_parent_logic (`KismetSystemLibrary.GetObjectName` _hitcomponent) _thispulse))
      (:`CastFailed`
        _))
    (return)
    (else
      (return))))

(fn `SendWater`
  (params (Box :type "BoxComponent Object Reference") (Quality :type Integer) (Pressure :type "Float (double-precision)"))
  (locals (NewLocalVar_0 :type "Box Structure" :default (struct :`Min` (1.0 1.0 1.0) :`Max` (5.0 5.0 5.0))) (NewLocalVar_1 :type "Array of EObjectTypeQuery Enum"))
  (bind (_returnvalue_x _returnvalue_y _returnvalue_z) (`KismetMathLibrary.BreakVector` (`SceneComponent.K2_GetComponentLocation` Box)))
  (bind (_returnvalue_x_2 _returnvalue_y_2 _returnvalue_z_2) (`KismetMathLibrary.BreakVector` (`SceneComponent.K2_GetComponentLocation` Box)))
  (if (`self.PlacedDown?`)
    (if (`KismetStringLibrary.EqualEqual_StrStr` (`KismetSystemLibrary.GetObjectName` (`PrimitiveComponent.GetMaterial` (`self.WaterPipe`) 0)) "M_Black")
      (`self.WaterColour` "/Game/Materials/M_Blue.M_Blue"))
    (`KismetSystemLibrary.K2_SetTimer` null "ResetWater" 1.5)
    (`self.IndicatorMove` (`KismetSystemLibrary.GetObjectName` Box))
    (bind _outhit (`KismetSystemLibrary.LineTraceSingle` (`KismetMathLibrary.MakeVector` (- _returnvalue_x_2 2.0) (- _returnvalue_y_2 2.0) (- _returnvalue_z_2 2.0)) (`KismetMathLibrary.MakeVector` (+ _returnvalue_x 2.0) (+ _returnvalue_y 2.0) (+ _returnvalue_z 2.0)) "TraceTypeQuery1" true))
    (bind (_bblockinghit _binitialoverlap _time _distance _location _impactpoint _normal _impactnormal _physmat _hitactor _hitcomponent) (`GameplayStatics.BreakHitResult` _outhit))
    (if (not (`KismetStringLibrary.EqualEqual_StrStr` (`KismetSystemLibrary.GetClassDisplayName` (`GameplayStatics.GetObjectClass` _hitactor)) "BP_PipeCork_C"))
      (bind _asbp_parent_water_item (cast `/Game/WorldObjects/Items/BuildItems/BP_ParentWaterItem` _hitactor)
        (:`then`
          (`self.WaterIn` _asbp_parent_water_item (`KismetSystemLibrary.GetObjectName` _hitcomponent) (`KismetMathLibrary.Clamp` Quality 1 10) (`KismetMathLibrary.FClamp` (- Pressure 1.0) 1.0 100.0)))
        (:`CastFailed`
          (`|SpawnActorFromClass` "/Game/WorldObjects/BP_ProjectileWater.BP_ProjectileWater_C" (`SceneComponent.K2_GetComponentToWorld` Box) "Undefined" "OverrideRootScale" null null)))
      (return))))

(fn `SignalIn`
  (params (Box :type String) (Active :type Boolean)))

(fn `ToggleWires`
  (params (Visible :type Boolean))
  (`SceneComponent.SetVisibility` (`self.ElectricCable`) Visible false)
  (`SceneComponent.SetVisibility` (`self.ElectricCable2`) Visible false)
  (`SceneComponent.SetVisibility` (`self.ElectricCable3`) Visible false)
  (`SceneComponent.SetVisibility` (`self.ElectricCable4`) Visible false)
  (`SceneComponent.SetVisibility` (`self.WaterPipe`) Visible false)
  (`SceneComponent.SetVisibility` (`self.WaterPipe2`) Visible false)
  (`SceneComponent.SetVisibility` (`self.Indicator1`) Visible false)
  (`SceneComponent.SetVisibility` (`self.Indicator2`) Visible false)
  (`SceneComponent.SetVisibility` (`self.Indicator3`) Visible false)
  (`SceneComponent.SetVisibility` (`self.Indicator4`) Visible false)
  (`SceneComponent.SetVisibility` (`self.Indicator5`) Visible false)
  (`SceneComponent.SetVisibility` (`self.Indicator6`) Visible false))

(fn `UnlockSignal`
  (locals (NewLocalVar_2 :type Boolean))
  (for _array_element (`self.Locks`)
    (`|VariableSetRef` _array_element)))

(fn `UnsetSignal`
  (set `self.SignalCount` 0)
  (set `self.SignalReset` true))

(fn `UnsetWater`
  (set `self.WaterOut?` false))

(fn `UserConstructionScript`
  (`parent.UserConstructionScript`)
  (set `self.Boxes` (`|MakeArray` (`self.Box1`) (`self.Box2`) (`self.Box3`) (`self.Box4`) (`self.Box5`) (`self.Box6`))))

(fn `WaterColour`
  (params (Colour :type "Material Object Reference"))
  (`PrimitiveComponent.SetMaterial` (`self.WaterPipe`) 0 Colour)
  (`PrimitiveComponent.SetMaterial` (`self.WaterPipe2`) 0 Colour))