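; Throwable grenade tool item that blasts a spherical hole in voxel terrain.
; Clicking with no target drops the item, launches it along the player camera's forward vector with extra vertical boost and starts a timed fuse.
; Once fused, any hit zeroes its velocity and disables gravity so it stops where it lands.
; When the fuse ends, it spawns BP_Explosion, carves the first overlapped VoxelWorld and destroys itself.
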(event `Explode`
  (bind _returnvalue (`self.K2_GetActorLocation`))
  (`KismetSystemLibrary.Delay` 3.0)
  (bind _outactors (`KismetSystemLibrary.SphereOverlapActors` _returnvalue 50.0 (`self.NewLocalVar_1`) "/Voxel/VoxelWorld.VoxelWorld_C"))
  (bind _returnvalue_2 (`|SpawnActorFromClass` "/Game/WorldObjects/Particles/BP_Explosion.BP_Explosion_C" (`self.GetTransform`) "Undefined" "OverrideRootScale" null null))
  (`ActorComponent.Activate` (`/Game/WorldObjects/Particles/BP_Explosion.ParticleSystem` _returnvalue_2) false)
  (bind (_asvoxel_world _bsuccess) (cast `VoxelWorld` (`|GetArrayItem` _outactors) :!pure true))
  (if _bsuccess
    (`VoxelSphereTools.RemoveSphere` _asvoxel_world _returnvalue 7.0 true true))
  (`self.K2_DestroyActor`))

(event `self.StaticMesh.OnComponentHit`
  (params (HitComponent :type "PrimitiveComponent Object Reference") (OtherActor :type "Actor Object Reference") (OtherComp :type "PrimitiveComponent Object Reference") (NormalImpulse :type "Vector Structure") (Hit :type "HitResult Structure (by ref)"))
  (if (`self.Fuse?`)
    (`PrimitiveComponent.SetAllPhysicsLinearVelocity` (`self.StaticMesh`) (0.0 0.0 0.0) false)
    (`PrimitiveComponent.SetEnableGravity` (`self.StaticMesh`) false)))

(event `self.OverrideClickNoTarget`
  (params (Controller :type "/Game/BP_GameController Object Reference") (`Hit Actor` :type "Actor Object Reference"))
  (bind (_returnvalue_x _returnvalue_y _returnvalue_z) (`KismetMathLibrary.BreakVector` (* (`SceneComponent.GetForwardVector` (`/Game/BP_GameCharacter.Camera` (cast `/Game/BP_GameCharacter` (`Controller.K2_GetPawn` (`GameplayStatics.GetPlayerController` 0)) :!pure true))) 1500.0)))
  (if (not (`self.Fuse?`))
    (`self.ItemDropped`)
    (`PrimitiveComponent.AddImpulse` (`self.StaticMesh`) (`KismetMathLibrary.MakeVector` _returnvalue_x _returnvalue_y (* _returnvalue_z 1.3)) "None" true)
    (set `self.Fuse?` true)
    (`self.Explode`)))

(fn `UserConstructionScript`
  (`parent.UserConstructionScript`))