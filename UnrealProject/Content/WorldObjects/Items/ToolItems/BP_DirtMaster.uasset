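; BP_DirtMaster is a tool item that works as a collision inspector when clicked with no target.
; The click override moves the mouse to the viewport center and runs Visibility traces under the cursor.
; One text render shows the hit component's collision object type, the other its response to the WorldStatic channel.
; The construction script only calls its parent.
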(event `/Game/WorldObjects/Items/BP_ParentItem.OverrideClickNoTarget`
  (params (Controller :type "/Game/BP_GameController Object Reference") (`Hit Actor` :type "Actor Object Reference"))
  (bind (_returnvalue_x _returnvalue_y) (`KismetMathLibrary.BreakVector2D` (`WidgetLayoutLibrary.GetViewportSize`)))
  (bind _returnvalue (`GameplayStatics.GetPlayerController` 0))
  (bind (_bblockinghit _binitialoverlap _time _distance _location _impactpoint _normal _impactnormal _physmat _hitactor _hitcomponent) (`GameplayStatics.BreakHitResult` (`PlayerController.GetHitResultUnderCursorByChannel` _returnvalue "TraceTypeQuery1" false)))
  (`PlayerController.SetMouseLocation` _returnvalue (`KismetMathLibrary.FTrunc` (/ _returnvalue_x 2.0)) (`KismetMathLibrary.FTrunc` (/ _returnvalue_y 2.0)))
  (`TextRenderComponent.K2_SetText` (`self.TextRender1`) (`KismetTextLibrary.Conv_NameToText` (`|GetEnumeratorName` (`PrimitiveComponent.GetCollisionResponseToChannel` _hitcomponent "ECC_WorldStatic"))))
  (`TextRenderComponent.K2_SetText` (`self.TextRender`) (`KismetTextLibrary.Conv_NameToText` (`|GetEnumeratorName` (`PrimitiveComponent.GetCollisionObjectType` _hitcomponent)))))

(fn `UserConstructionScript`
  (`parent.UserConstructionScript`))