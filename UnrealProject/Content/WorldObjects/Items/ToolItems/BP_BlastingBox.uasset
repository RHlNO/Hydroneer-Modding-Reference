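; Blasting box tool item that, when activated by mouse, explodes and carves a hole in the voxel terrain.
; Activation checks for an overlapping VoxelWorld, fires its particle systems, then waits briefly before spawning and triggering a BP_Explosion.
; It then removes a sphere from any voxel world found at the start and destroys itself.
; The construction script caches the first CastleSpawn as CastleControl and disables auto-activation on one particle system.
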(event `/Game/WorldObjects/Items/BP_ParentItem.OverrideMouseActivated`
  (params (Component :type "ActorComponent Object Reference"))
  (bind _returnvalue (`self.K2_GetActorLocation`))
  (bind (_outactors _returnvalue_2) (`KismetSystemLibrary.SphereOverlapActors` _returnvalue 30.0 (`self.NewLocalVar_1`) "/Voxel/VoxelWorld.VoxelWorld_C"))
  (`ActorComponent.Activate` (`self.ParticleSystem`) false)
  (`ActorComponent.Activate` (`self.ParticleSystem4`) false)
  (`ActorComponent.Activate` (`self.ParticleSystem7`) false)
  (`ActorComponent.Activate` (`self.ParticleSystem3`) false)
  (`ActorComponent.Activate` (`self.ParticleSystem8`) false)
  (`ActorComponent.Activate` (`self.ParticleSystem6`) false)
  (`ActorComponent.Activate` (`self.ParticleSystem2`) false)
  (`ActorComponent.Activate` (`self.ParticleSystem1`) false)
  (`ActorComponent.Activate` (`self.ParticleSystem9`) false)
  (`ActorComponent.Activate` (`self.ParticleSystem10`) false)
  (`ActorComponent.Activate` (`self.ParticleSystem5`) false)
  (`KismetSystemLibrary.Delay` 2.0)
  (bind _returnvalue_3 (`|SpawnActorFromClass` "/Game/WorldObjects/Particles/BP_Explosion.BP_Explosion_C" (`self.GetTransform`) "Undefined" "OverrideRootScale" null null))
  (`ActorComponent.Activate` (`/Game/WorldObjects/Particles/BP_Explosion.ParticleSystem` _returnvalue_3) false)
  (if _returnvalue_2
    (`VoxelSphereTools.RemoveSphere` (cast `VoxelWorld` (`|GetArrayItem` _outactors) :!pure true) _returnvalue 30.0 true true))
  (`self.K2_DestroyActor`))

(fn `UserConstructionScript`
  (`parent.UserConstructionScript`)
  (bind _outactors (`GameplayStatics.GetAllActorsOfClass` "/Game/ModIndex/CastleSpawn.CastleSpawn_C"))
  (set `self.CastleControl` (`|GetArrayItem` _outactors))
  (`ActorComponent.SetAutoActivate` (`self.ParticleSystem`) false))