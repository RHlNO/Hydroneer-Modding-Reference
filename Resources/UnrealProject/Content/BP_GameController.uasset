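; BP_GameController handles the player's left-click interaction with world resources and items.
; A click recenters the mouse and traces under the cursor on Visibility, storing a BP_ParentResource as CarryingItem or forwarding the hit component to BP_ParentItem's OverrideMouseActivated.
; PickUpItem only resets the crosshair.
; Other functions, covering saving, UI, vehicle recall, unsticking, music, dirt digging and dropping, are empty stubs.
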(event `InputAction|PlayerForward`
  (params (Key :type "Key Structure")))

(event `InputAction|PlayerBackward`
  (params (Key :type "Key Structure")))

(event `InputAction|PlayerLeft`
  (params (Key :type "Key Structure")))

(event `InputAction|PlayerRight`
  (params (Key :type "Key Structure")))

(event `InputAction|LeftClick`
  (params (Key :type "Key Structure"))
  (bind (_bblockinghit _binitialoverlap _time _distance _location _impactpoint _normal _impactnormal _physmat _hitactor _hitcomponent) (`GameplayStatics.BreakHitResult` (`self.GetHitResultUnderCursorByChannel` "TraceTypeQuery1" false)))
  (:`Pressed`
    (`self.CenterMouse`)
    (bind _asbp_parent_resource (cast `/Game/WorldObjects/Items/ResourceItems/BP_ParentResource` _hitactor)
      (:`then`
        (set `self.CarryingItem` _asbp_parent_resource))
      (:`CastFailed`
        (bind _asbp_parent_item (cast `/Game/WorldObjects/Items/BP_ParentItem` _hitactor))
        (`/Game/WorldObjects/Items/BP_ParentItem.OverrideMouseActivated` _asbp_parent_item _hitcomponent)))))

(fn `CenterMouse`
  (bind (_returnvalue_x _returnvalue_y) (`KismetMathLibrary.BreakVector2D` (`WidgetLayoutLibrary.GetViewportSize`)))
  (`self.SetMouseLocation` (`GameplayStatics.GetPlayerController` 0) (`KismetMathLibrary.FTrunc` (/ _returnvalue_x 2.0)) (`KismetMathLibrary.FTrunc` (/ _returnvalue_y 2.0))))

(fn `CloseAllUI`)

(fn `CrosshairTrace`)

(fn `DigCheckForRelicPlants`
  (params (`Actor Hit` :type "Actor Object Reference")))

(fn `DropItem`)

(fn `LevelTerrain`)

(fn `MoveDirt`
  (params (`PickUp?` :type Boolean) (Radius :type "Float (double-precision)")))

(fn `MovePlayerToNearestUnstickPoint`)

(fn `PickUpItem`
  (params (Item :type "Actor Object Reference"))
  (set `self.CurrentCrosshair` 0))

(fn `RecallVehicle`)

(fn `RemoveDirtByLocation`
  (params (Location :type "Vector Structure") (Radius :type "Float (double-precision)")))

(fn `RemoveDirtLine`)

(fn `ReturnNoActivation`
  (params (NewParam :type "Actor Object Reference")))

(fn `SaveGame`)

(fn `ToggleMusic`
  (params (`Play?` :type Boolean)))

(fn `UserConstructionScript`)