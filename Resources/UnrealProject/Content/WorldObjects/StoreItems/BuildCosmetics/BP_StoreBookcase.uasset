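; BP_StoreBookcase is a store build-cosmetic bookcase that also makes sure a configured set of actor classes exists in the world.
; From BeginPlay, a looping timer polls the player's BP_GameController until its movement mode is the first enum value.
; It then clears the timer and spawns each SpawnClasses entry that has no existing instance, ignoring collisions.
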(event `self.ReceiveBeginPlay`
  (bind _returnvalue (`KismetSystemLibrary.K2_SetTimerDelegate` (delegate `BeginSpanwers`) 1.5 true)))

(event `BeginSpanwers`
  (if (== (`/Game/BP_GameController.CurrentMovementMode` (cast `/Game/BP_GameController` (`GameplayStatics.GetPlayerController` 0) :!pure true)) 0)
    (`|ExecutionSequence`
      (:`then_0`
        (`KismetSystemLibrary.K2_ClearAndInvalidateTimerHandle` (stale `self.ReceiveBeginPlay` _returnvalue)))
      (:`then_1`
        (for _array_element (`self.SpawnClasses`)
          (bind _outactors (`GameplayStatics.GetAllActorsOfClass` _array_element))
          (if (== (`KismetArrayLibrary.Array_Length` _outactors) 0)
            (`|SpawnActorFromClass` _array_element (`KismetMathLibrary.MakeTransform` (0.0 0.0 0.0)) "AlwaysSpawn" "OverrideRootScale" null null)))))))

(fn `UserConstructionScript`
  (`parent.UserConstructionScript`))