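; BP_StorePlinth is a store world object that makes sure a BP_StoreGemGrinder exists in the level.
; On BeginPlay it starts a looping timer that polls the first BP_GameController until its CurrentMovementMode is the zero value.
; It then spawns the grinder at a hardcoded world transform if none is present, and clears the timer.
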(event `self.ReceiveBeginPlay`
  (bind _returnvalue (`KismetSystemLibrary.K2_SetTimerDelegate` (delegate `BeginSpanwers`) 1.5 true)))

(event `BeginSpanwers`
  (if (== (`/Game/BP_GameController.CurrentMovementMode` (cast `/Game/BP_GameController` (`GameplayStatics.GetPlayerController` 0) :!pure true)) 0)
    (bind _outactors (`GameplayStatics.GetAllActorsOfClass` "/Game/WorldObjects/StoreItems/EquipmentToolStores/BP_StoreGemGrinder.BP_StoreGemGrinder_C"))
    (if (== (`KismetArrayLibrary.Array_Length` _outactors) 0)
      (`|SpawnActorFromClass` "/Game/WorldObjects/StoreItems/EquipmentToolStores/BP_StoreGemGrinder.BP_StoreGemGrinder_C" (`KismetMathLibrary.MakeTransform` (12388.0 30953.199219 511.0) (struct :`Yaw` -50.0)) "AlwaysSpawn" "OverrideRootScale" null null))
    (`KismetSystemLibrary.K2_ClearAndInvalidateTimerHandle` (stale `self.ReceiveBeginPlay` _returnvalue))))

(fn `UserConstructionScript`
  (`parent.UserConstructionScript`))