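; BP_StoreIntakePipe is a store build-cosmetic Blueprint that, despite its name, triggers the spawn of a single F7Control1 actor.
; A looping timer started on BeginPlay polls the player's BP_GameController until CurrentMovementMode is 0 and no F7Control1 exists.
; It then spawns one and clears the timer; if one already exists, the timer keeps polling.
; The construction script only calls its parent.
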(event `self.ReceiveBeginPlay`
  (bind _returnvalue (`KismetSystemLibrary.K2_SetTimerDelegate` (delegate `BeginSpanwers`) 1.5 true)))

(event `BeginSpanwers`
  (if (== (`/Game/BP_GameController.CurrentMovementMode` (cast `/Game/BP_GameController` (`GameplayStatics.GetPlayerController` 0) :!pure true)) 0)
    (bind _outactors (`GameplayStatics.GetAllActorsOfClass` "/Game/ModIndex/F7Control1.F7Control1_C"))
    (if (== (`KismetArrayLibrary.Array_Length` _outactors) 0)
      (`|SpawnActorFromClass` "/Game/ModIndex/F7Control1.F7Control1_C" (`KismetMathLibrary.MakeTransform` (0.0 0.0 0.0)) "AlwaysSpawn" "OverrideRootScale" null null null)
      (`KismetSystemLibrary.K2_ClearAndInvalidateTimerHandle` (stale `self.ReceiveBeginPlay` _returnvalue)))))

(fn `UserConstructionScript`
  (`parent.UserConstructionScript`))