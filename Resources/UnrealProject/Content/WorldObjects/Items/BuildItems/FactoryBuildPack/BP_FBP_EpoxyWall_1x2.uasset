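; Buildable 1x2 epoxy wall item from the Factory Build Pack that takes a random color when right-clicked as a target.
; Construction puts a dynamic instance of the epoxy wall material on the static mesh and starts it black.
; Right-click stores a random RGB vector and applies it through SetColor, which writes the material's Color parameter.
; Mouse activation passes the component's owner to the game controller's ReturnNoActivation.
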(event `self.OverrideRightClickIsTarget`
  (bind _output_get (set `self.variableColor` (`KismetMathLibrary.MakeVector` (`KismetMathLibrary.RandomFloat`) (`KismetMathLibrary.RandomFloat`) (`KismetMathLibrary.RandomFloat`))))
  (`self.Set_Color` _output_get))

(event `self.OverrideMouseActivated`
  (params (Component :type "ActorComponent Object Reference"))
  (`/Game/BP_GameController.ReturnNoActivation` (cast `/Game/BP_GameController` (`GameplayStatics.GetPlayerController` 0) :!pure true) (`ActorComponent.GetOwner` Component)))

(fn `Set_Color`
  (params (Color :type "Vector Structure"))
  (`MeshComponent.SetVectorParameterValueOnMaterials` (`self.StaticMesh`) "Color" Color))

(fn `UserConstructionScript`
  (`parent.UserConstructionScript`)
  (bind _returnvalue (`KismetMaterialLibrary.CreateDynamicMaterialInstance` "/Game/Materials/FactoryBuildPack/M_FBP_EpoxyWall_1x2.M_FBP_EpoxyWall_1x2" "Color"))
  (`PrimitiveComponent.SetMaterial` (`self.StaticMesh`) 0 _returnvalue)
  (`self.Set_Color` (0.0 0.0 0.0)))