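; Placeable hanging light fixture build item that builds its own chain up toward whatever is above it.
; On placement it turns on both point lights, box-traces upward from its center point, and spawns locked chain segment actors at even intervals to span the gap.
; Pickup switches the lights off and destroys the chain, while right-click toggles the lights.
; Mouse activation is passed to the game controller's ReturnNoActivation.
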(event `self.OverridePlacedDown`
  (bind _centerpoint (`self.CenterPoint`))
  (bind _returnvalue (`SceneComponent.K2_GetComponentToWorld` _centerpoint))
  (`SceneComponent.SetVisibility` (`self.PointLight1`) true false)
  (`SceneComponent.SetVisibility` (`self.PointLight2`) true false)
  (`KismetArrayLibrary.Array_Clear` (`self.ChainArray`))
  (bind _outhit (`KismetSystemLibrary.BoxTraceSingle` (`KismetMathLibrary.MakeVector` (.x (.location _returnvalue)) (.y (.location _returnvalue)) (.z (.location _returnvalue))) (`KismetMathLibrary.MakeVector` (.x (.location _returnvalue)) (.y (.location _returnvalue)) (+ (.z (.location _returnvalue)) 1000.0)) (25.0 25.0 25.0) (struct) "TraceTypeQuery1"))
  (bind (_returnvalue_x _returnvalue_y _returnvalue_z) (`KismetMathLibrary.BreakVector` (- (`.Location` (`GameplayStatics.BreakHitResult` _outhit)) (`SceneComponent.K2_GetComponentLocation` _centerpoint))))
  (for _index (range (+ (`KismetMathLibrary.FCeil` (/ (- _returnvalue_z 50.0) 100.0)) 1))
    (if (> _index 0)
      (bind _returnvalue_2 (`|SpawnActorFromClass` "/Game/WorldObjects/Items/BuildItems/FactoryBuildPack/BP_FBP_FixtureChain.BP_FBP_FixtureChain_C" (`KismetMathLibrary.MakeTransform` (`KismetMathLibrary.MakeVector` (.x (.location _returnvalue)) (.y (.location _returnvalue)) (+ (.z (.location _returnvalue)) (* _index 100.0))) (.rotation _returnvalue)) "AlwaysSpawn" "OverrideRootScale" null true false false true false false false false false true false false "" "" 0 "NewEnumerator7" null))
      (`KismetArrayLibrary.Array_Add` (`self.ChainArray`) _returnvalue_2))))

(event `/Game/WorldObjects/Items/BP_ParentItem.OverrideRightClickIsTarget`
  (bind _pointlight1 (`self.PointLight1`))
  (bind _pointlight2 (`self.PointLight2`))
  (if (`SceneComponent.IsVisible` _pointlight1)
    (`SceneComponent.SetVisibility` _pointlight1 false false)
    (`SceneComponent.SetVisibility` _pointlight2 false false)
    (else
      (`SceneComponent.SetVisibility` _pointlight1 true false)
      (`SceneComponent.SetVisibility` _pointlight2 true false))))

(event `/Game/WorldObjects/Items/BP_ParentItem.OverridePickedup`
  (`SceneComponent.SetVisibility` (`self.PointLight1`) false false)
  (`SceneComponent.SetVisibility` (`self.PointLight2`) false false)
  (for _array_element (`self.ChainArray`)
    (`self.K2_DestroyActor` _array_element)))

(event `/Game/WorldObjects/Items/BP_ParentItem.OverrideMouseActivated`
  (params (Component :type "ActorComponent Object Reference"))
  (`/Game/BP_GameController.ReturnNoActivation` (cast `/Game/BP_GameController` (`GameplayStatics.GetPlayerController` 0) :!pure true) (`ActorComponent.GetOwner` Component)))

(fn `UserConstructionScript`
  (`parent.UserConstructionScript`))