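; Placeable Hydronix build item that reacts to incoming water by launching a BP_MeatballEater across the terrain.
; Waterin, once placed, flags water briefly and steps along the CenterPoint-to-SecondPoint direction, sphere-tracing downward for VoxelWorld ground.
; If ground ends within the step limit, it spawns the eater at SecondPoint and sends it to the last grounded step.
; A timed Fired flag sets the launch cooldown.
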(event `WaterGone`
  (set `self.Water?` false))

(event `self.WaterIn`
  (params (Box :type String) (WaterQuality :type Integer) (WaterPressure :type "Float (single-precision)"))
  (bind _counter (`self.Counter`))
  (bind _returnvalue (+ (* (`self.Distance`) (`self.Counter`)) (`SceneComponent.K2_GetComponentLocation` (`self.CenterPoint`))))
  (if (`self.PlacedDown?`)
    (set `self.Water?` true)
    (`KismetSystemLibrary.K2_SetTimerDelegate` (delegate `WaterGone`) 1.5)
    (if (not (`self.Fired?`))
      (set `self.Distance` (- (`SceneComponent.K2_GetComponentLocation` (`self.SecondPoint`)) (`SceneComponent.K2_GetComponentLocation` (`self.CenterPoint`))))
      (set `self.Hit?` true)
      (while (and (< (`self.Counter`) 50) (`self.Hit?`))
        (bind _outhits (`KismetSystemLibrary.SphereTraceMultiForObjects` (+ _returnvalue 1) (`KismetMathLibrary.MakeVector` (.x _returnvalue) (.y _returnvalue) -1000.0) 5.0 (`self.NewVar_0_0`)))
        (set `self.Dirt?` false)
        (for _array_element _outhits
          (cast `VoxelWorld` (`.HitActor` (`GameplayStatics.BreakHitResult` _array_element)))
          (set `self.HitDirt` _array_element)
          (set `self.Dirt?` true))
        (if (`self.Dirt?`)
          (`/Engine/EditorBlueprintResources/StandardMacros.IncrementInt` _counter)
          (else
            (set `self.Hit?` false)
            (`/Engine/EditorBlueprintResources/StandardMacros.DecrementInt` _counter))))
      (if (or (< (`self.Counter`) 1) (`self.Hit?`))
        (set `self.Counter` 1)
        (else
          (set `self.Fired?` true)
          (`KismetSystemLibrary.K2_SetTimerDelegate` (delegate `ResetFire`) 30.0)
          (bind _returnvalue_2 (`|SpawnActorFromClass` "/Game/WorldObjects/BP_MeatballEater.BP_MeatballEater_C" (`SceneComponent.K2_GetComponentToWorld` (`self.SecondPoint`)) "Undefined" "OverrideRootScale" null null))
          (`/Game/WorldObjects/BP_MeatballEater.TravelTo` _returnvalue_2 (+ (* (`self.Distance`) (`self.Counter`)) (`SceneComponent.K2_GetComponentLocation` (`self.CenterPoint`))))
          (set `self.Counter` 1))))))

(event `ResetFire`
  (set `self.Fired?` false))

(fn `UserConstructionScript`
  (`parent.UserConstructionScript`))