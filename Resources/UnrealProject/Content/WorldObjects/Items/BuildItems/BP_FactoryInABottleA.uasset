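; BP_FactoryInABottleA is a placeable build item that deploys a prefabricated factory from the world.
; Once placed, clicking its button animates a press, spawns every actor listed in a build DataTable relative to CenterPoint, then destroys the item.
; Clicking its lever plays a timeline that rotates it and toggles preview mode.
; In this graph, preview only sets the PreviewOn and Locked flags, without spawning preview visuals.
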(event `self.OverridePlacedDown`
  (if (`self.PlacedDown?`)
    (set `self.PreviewOn?` false)
    (`SceneComponent.K2_SetRelativeRotation` :`self` (`self.PreviewLever`)))
  (`parent.OverridePlacedDown`))

(event `ButtonReset`
  (`StaticMeshComponent.SetStaticMesh` (`self.PlacementButton`) "/Game/Meshes/UsedItems/MapItems/SM_ButtonUp.SM_ButtonUp"))

(event `/Game/WorldObjects/Items/BP_ParentItem.OverrideMouseActivated`
  (params (Component :type "ActorComponent Object Reference"))
  (bind _previewlever (`self.PreviewLever`))
  (if (`self.PlacedDown?`)
    (switch `string` (`KismetSystemLibrary.GetObjectName` Component)
      (:`PlacementButton`
        (`StaticMeshComponent.SetStaticMesh` (`self.PlacementButton`) "/Game/Meshes/UsedItems/MapItems/SM_ButtonDown.SM_ButtonDown")
        (`GameplayStatics.PlaySound2D` "/Game/Sound/Player/Button_Press.Button_Press" 1.0 1.0 0.0 null null)
        (`KismetSystemLibrary.K2_SetTimerDelegate` (delegate `ButtonReset`) 0.5)
        (if (`self.PreviewOn?`)
          (`self.StopPreview`))
        (`self.BuildFactory`))
      (:`PreviewLever`
        (bind (_direction _newtrack_0 _newtrack_1) (`Timeline|LeverTimeline` :!via `PlayFromStart`)
          (:`Update`
            (if (`self.PreviewOn?`)
              (`SceneComponent.K2_SetRelativeRotation` _previewlever (`KismetMathLibrary.MakeRotator` 0.0 _newtrack_1) false false)
              (else
                (`SceneComponent.K2_SetRelativeRotation` _previewlever (`KismetMathLibrary.MakeRotator` 0.0 _newtrack_0) false false))))
          (:`Finished`
            (if (`self.PreviewOn?`)
              (`self.StopPreview`)
              (else
                (`self.ShowPreview`)))))))))

(event `ShowPreview`
  (set `self.Locked?` true)
  (set `self.PreviewOn?` true))

(event `StopPreview`
  (set `self.PreviewOn?` false)
  (set `self.Locked?` false))

(event `BuildFactory`
  (bind _returnvalue (`SceneComponent.K2_GetComponentToWorld` (`self.CenterPoint`)))
  (bind _outrownames (`DataTableFunctionLibrary.GetDataTableRowNames` "/Game/DT_FactoryInABottle_BuildData.DT_FactoryInABottle_BuildData"))
  (for _array_element _outrownames
    (bind _returnvalue_2 (`|GetDataTableRow` "/Game/DT_FactoryInABottle_BuildData.DT_FactoryInABottle_BuildData" _array_element)
      (:`then`
        (bind (_actorclass _relativetransform) (break `/Game/Struct_FactoryInABottle_BuildData` _returnvalue_2))
        (`|SpawnActorFromClass` _actorclass (`KismetMathLibrary.MakeTransform` (`KismetMathLibrary.TransformLocation` _returnvalue (.location _relativetransform)) (`KismetMathLibrary.TransformRotation` _returnvalue (.rotation _relativetransform)) (.scale _relativetransform)) "Undefined" "OverrideRootScale" null null))))
  (`self.K2_DestroyActor`))

(fn `UserConstructionScript`
  (`parent.UserConstructionScript`)
  (set `self.ExtraMeshes` (`|MakeArray` (`self.PlacementButton`) (`self.PreviewLever`))))