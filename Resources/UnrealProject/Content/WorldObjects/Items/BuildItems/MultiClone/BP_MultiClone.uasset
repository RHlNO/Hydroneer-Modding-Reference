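; BP_MultiClone is a build item world object that serves as the access point for the multi-clone menu.
; Its right-click target override creates UI_MultiCloneMenu, adds it to the viewport, shows the mouse cursor and switches input to UI only.
; BeginPlay is disabled, Tick and construction only call the parent, and two chains that toggle its four point lights are left unconnected.
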(event `self.ReceiveTick`
  (params (DeltaSeconds :type "Float (single-precision)"))
  (`parent.ReceiveTick` DeltaSeconds))

(event `/Game/WorldObjects/Items/BP_ParentItem.OverrideRightClickIsTarget`
  (bind _returnvalue (`GameplayStatics.GetPlayerController` 0))
  (bind _returnvalue_2 (`|CreateWidget` "/Game/UI/UI_MultiCloneMenu.UI_MultiCloneMenu_C"))
  (`UserWidget.AddToViewport` _returnvalue_2 0)
  (set `PlayerController.bShowMouseCursor` true _returnvalue)
  (`WidgetBlueprintLibrary.SetInputMode_UIOnlyEx` _returnvalue _returnvalue_2))

(fn `UserConstructionScript`
  (`parent.UserConstructionScript`))