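; BP_FBP_LightFixture is a placeable build item for a light fixture that generates its own hanging chain when placed.
; On placement, it box-traces upward from CenterPoint and spawns locked BP_FBP_FixtureChain segments at fixed vertical intervals, with the count derived from the hit height.
; The segments are stored in ChainArray and destroyed when the fixture is picked up.
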(event `self.OverridePlacedDown`
  (bind _centerpoint (`self.CenterPoint`))
  (bind (_returnvalue_x _returnvalue_y _returnvalue_z) (`KismetMathLibrary.BreakVector` (`SceneComponent.K2_GetComponentLocation` _centerpoint)))
  (`KismetArrayLibrary.Array_Clear` (`self.ChainArray`))
  (bind _outhit (`KismetSystemLibrary.BoxTraceSingle` (`KismetMathLibrary.MakeVector` _returnvalue_x _returnvalue_y _returnvalue_z) (`KismetMathLibrary.MakeVector` _returnvalue_x _returnvalue_y (+ _returnvalue_z 1000.0)) (25.0 25.0 25.0) (struct) "TraceTypeQuery1"))
  (bind (_returnvalue_x_2 _returnvalue_y_2 _returnvalue_z_2) (`KismetMathLibrary.BreakVector` (- (`.Location` (`GameplayStatics.BreakHitResult` _outhit)) (`SceneComponent.K2_GetComponentLocation` _centerpoint))))
  (for _index (range (+ (`KismetMathLibrary.FCeil` (/ (- _returnvalue_z_2 50.0) 100.0)) 1))
    (if (> _index 0)
      (bind _returnvalue (`|SpawnActorFromClass` "/Game/WorldObjects/Items/BuildItems/BP_FBP_FixtureChain.BP_FBP_FixtureChain_C" (`KismetMathLibrary.MakeTransform` (`KismetMathLibrary.MakeVector` _returnvalue_x _returnvalue_y (+ _returnvalue_z (* _index 100.0)))) "AlwaysSpawn" "OverrideRootScale" null true false false true false false false false false true false false "" "" 0 "NewEnumerator7" null))
      (`KismetArrayLibrary.Array_Add` (`self.ChainArray`) _returnvalue))))

(event `/Game/WorldObjects/Items/BP_ParentItem.OverridePickedup`
  (for _array_element (`self.ChainArray`)
    (`self.K2_DestroyActor` _array_element)))

(fn `UserConstructionScript`
  (`parent.UserConstructionScript`))