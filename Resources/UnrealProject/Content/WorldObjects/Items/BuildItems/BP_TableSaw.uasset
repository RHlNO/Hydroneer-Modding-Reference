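; Placeable table saw, powered by a short-lived water input, that cuts a piece of a chosen size from a "Bar" resource.
; Clicking the mesh clamps a carried bar; clickable digit boxes set the size, with the last digit toggling between 0 and 5.
; While water runs, the button checks the clamped bar via a short trace, animates the cut, spawns the piece and deducts its size plus 5% from the bar.
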(event `CustomEvent_0`
  (set `self.Water?` false))

(event `self.WaterIn`
  (params (Box :type String) (WaterQuality :type Integer) (WaterPressure :type "Float (single-precision)"))
  (if (`self.PlacedDown?`)
    (set `self.Water?` true)
    (`KismetSystemLibrary.K2_SetTimerDelegate` (delegate `CustomEvent_0`) 1.5)
    (`Timeline|Timeline_1` :!via `PlayFromStart`
      (:`Update`
        (`SceneComponent.K2_AddLocalRotation` (`self.Saw`) (struct :`Roll` -0.5) false false)))))

(event `self.OverrideMouseActivated`
  (params (Component :type "ActorComponent Object Reference"))
  (bind _clampbox (`self.ClampBox`))
  (bind _textdecimal (`self.TextDecimal`))
  (bind (_returnvalue_x _returnvalue_y _returnvalue_z) (`KismetMathLibrary.BreakVector` (`SceneComponent.K2_GetComponentLocation` _clampbox)))
  (bind (_returnvalue_x_2 _returnvalue_y_2 _returnvalue_z_2) (`KismetMathLibrary.BreakVector` (`SceneComponent.K2_GetComponentLocation` _clampbox)))
  (bind _asbp_game_controller (cast `/Game/BP_GameController` (`GameplayStatics.GetPlayerController` 0)))
  (bind _output_get (set `self.Controller` _asbp_game_controller))
  (bind (_outhit _returnvalue) (`KismetSystemLibrary.LineTraceSingle` (`KismetMathLibrary.MakeVector` (- _returnvalue_x_2 2.0) (- _returnvalue_y_2 2.0) (- _returnvalue_z_2 2.0)) (`KismetMathLibrary.MakeVector` (+ _returnvalue_x 2.0) (+ _returnvalue_y 2.0) (+ _returnvalue_z 2.0)) "TraceTypeQuery1"))
  (switch `string` (`KismetSystemLibrary.GetObjectName` Component)
    (:`StaticMesh`
      (if (not _returnvalue)
        (bind _asbp_parent_resource (cast `/Game/WorldObjects/Items/ResourceItems/BP_ParentResource` (`/Game/BP_GameController.CarryingItem` _output_get)))
        (if (`KismetStringLibrary.Contains` (`KismetSystemLibrary.GetObjectName` _asbp_parent_resource) "Bar")
          (set `/Game/BP_GameController.CarryingItem` null (`self.Controller`))
          (set `/Game/WorldObjects/Items/BP_ParentItem.Carryer` null _asbp_parent_resource)
          (`self.K2_AttachToComponent` _asbp_parent_resource (`self.Clamp`) "None" "KeepRelative" "KeepRelative" "KeepRelative" false)
          (`self.K2_SetActorRelativeTransform` _asbp_parent_resource (`KismetMathLibrary.MakeTransform` (-7.0 -22.700001 -3.0) (struct) (2.54 2.54 2.54)) false false)
          (set `/Game/WorldObjects/Items/BP_ParentItem.BeingCarried?` false _asbp_parent_resource)
          (set `/Game/WorldObjects/Items/BP_ParentItem.Stored?` true _asbp_parent_resource)
          (set `/Game/WorldObjects/Items/BP_ParentItem.BeingStoredBy` self _asbp_parent_resource))))
    (:`Button`
      (if (and (`self.PlacedDown?`) (`self.Water?`))
        (bind _asbp_parent_resource_2 (cast `/Game/WorldObjects/Items/ResourceItems/BP_ParentResource` (`.HitActor` (`GameplayStatics.BreakHitResult` _outhit))))
        (if (and (`KismetStringLibrary.Contains` (`KismetSystemLibrary.GetObjectName` _asbp_parent_resource_2) "Bar") (> (- (`/Game/WorldObjects/Items/ResourceItems/BP_ParentResource.Size` _asbp_parent_resource_2) (* (+ (* (`self.Hundreds`) 100.0) (* (`self.Tens`) 10.0) (`self.Units`) (* (`self.Tenths`) 0.1)) 1.05)) 0.0))
          (`KismetSystemLibrary.K2_SetTimerDelegate` (delegate `CustomEvent_1`) 0.5)
          (bind (_direction _newtrack_2) (`Timeline|Timeline_0` :!via `PlayFromStart`)
            (:`Update`
              (`SceneComponent.K2_AddLocalRotation` (`self.Saw`) (struct :`Roll` -6.0) false false)
              (`SceneComponent.K2_SetRelativeLocation` (`self.Clamp`) (`KismetMathLibrary.MakeVector` 15.6 _newtrack_2 -1.2) false false))))))
    (:`HundredsBox`
      (bind _newnum (`self.IncreaseNumber` (`self.Hundreds`) (`self.TextHundred`)))
      (set `self.Hundreds` _newnum))
    (:`TensBox`
      (bind _newnum_2 (`self.IncreaseNumber` (`self.Tens`) (`self.TextTen`)))
      (set `self.Tens` _newnum_2))
    (:`UnitsBox`
      (bind _newnum_3 (`self.IncreaseNumber` (`self.Units`) (`self.TextUnit`)))
      (set `self.Units` _newnum_3))
    (:`TenthsBox`
      (`/Engine/EditorBlueprintResources/StandardMacros.FlipFlop`
        (:`A`
          (set `self.Tenths` 5.0)
          (`TextRenderComponent.K2_SetText` _textdecimal (`KismetTextLibrary.Conv_StringToText` "5")))
        (:`B`
          (set `self.Tenths` 0.0)
          (`TextRenderComponent.K2_SetText` _textdecimal (`KismetTextLibrary.Conv_StringToText` "0")))))))

(event `CustomEvent_1`
  (bind _returnvalue (+ (* (`self.Hundreds`) 100.0) (* (`self.Tens`) 10.0) (`self.Units`) (* (`self.Tenths`) 0.1)))
  (bind _returnvalue_2 (`|SpawnActorFromClass` (`GameplayStatics.GetObjectClass` (stale `self.OverrideMouseActivated` _asbp_parent_resource_2)) (`SceneComponent.K2_GetComponentToWorld` (`self.SpawnBox`)) "AdjustIfPossibleButAlwaysSpawn" "OverrideRootScale" null _returnvalue 0 false false true false false "" "" 0 "(INVALID)" null))
  (`self.OverrideLoaded` _returnvalue_2)
  (`self.ItemDropped` _returnvalue_2)
  (set `/Game/WorldObjects/Items/ResourceItems/BP_ParentResource.Size` (- (`/Game/WorldObjects/Items/ResourceItems/BP_ParentResource.Size` (stale `self.OverrideMouseActivated` _asbp_parent_resource_2)) (* _returnvalue 1.05)) (stale `self.OverrideMouseActivated` _asbp_parent_resource_2)))

(event `self.ClampBox.OnComponentEndOverlap`
  (params (OverlappedComponent :type "PrimitiveComponent Object Reference") (OtherActor :type "Actor Object Reference") (OtherComp :type "PrimitiveComponent Object Reference") (OtherBodyIndex :type Integer))
  (bind _asbp_parent_resource (cast `/Game/WorldObjects/Items/ResourceItems/BP_ParentResource` OtherActor))
  (`self.OverrideLoaded` _asbp_parent_resource))

(fn `IncreaseNumber`
  (params (Input :type "Float (double-precision)") (NewParam :type "TextRenderComponent Object Reference"))
  (returns (NewNum :type "Float (double-precision)"))
  (bind _result (`/Engine/EditorBlueprintResources/StandardMacros.IncrementFloat` Input)
    (:`  `
      (bind _returnvalue (mod _result 10.0))
      (`TextRenderComponent.K2_SetText` NewParam (`KismetTextLibrary.Conv_DoubleToText` _returnvalue "HalfToEven"))
      (return _returnvalue))))

(fn `UserConstructionScript`
  (`parent.UserConstructionScript`)
  (set `self.ExtraMeshes` (`|MakeArray` (`self.Clamp`) (`self.Pin`) (`self.Saw`) (`self.Button`))))