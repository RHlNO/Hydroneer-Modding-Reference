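; Placeable water-powered gem grinder build item that turns uncut emeralds, rubies and sapphires into their finished gems.
; Incoming water, once placed, spins both wheels via a timeline and keeps the grinder active until a short timer, restarted on each delivery, expires.
; Uncut gems overlapping the active grinder are replaced by dropped finished gems, their size scaled by water pressure.
; Water quality is stored but not used in grinding.
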(event `CustomEvent_0`
  (set `self.Water?` false))

(event `self.WaterIn`
  (params (Box :type String) (WaterQuality :type Integer) (WaterPressure :type "Float (single-precision)"))
  (if (`self.PlacedDown?`)
    (set `self.Quality` WaterQuality)
    (set `self.Pressure` WaterPressure)
    (set `self.Water?` true)
    (`KismetSystemLibrary.K2_SetTimerDelegate` (delegate `CustomEvent_0`) 1.5)
    (`self.WheelSpin`)))

(event `WheelSpin`
  (`Timeline|Timeline_0` :`NewTime` 1.0 :!via `PlayFromStart`
    (:`Update`
      (`SceneComponent.K2_AddLocalRotation` (`self.WheelOne`) (`KismetMathLibrary.MakeRotator` 0.0 0.0 -4.0) false false)
      (`SceneComponent.K2_AddLocalRotation` (`self.WheelTwo`) (`KismetMathLibrary.MakeRotator` 0.0 0.0 -4.0) false false))))

(event `self.GemGrind.OnComponentBeginOverlap`
  (params (OverlappedComponent :type "PrimitiveComponent Object Reference") (OtherActor :type "Actor Object Reference") (OtherComp :type "PrimitiveComponent Object Reference") (OtherBodyIndex :type Integer) (bFromSweep :type Boolean) (SweepResult :type "HitResult Structure (by ref)"))
  (bind _returnvalue (`KismetMathLibrary.MapRangeClamped` (`self.Pressure`) 0.0 100.0 0.5 1.1))
  (bind _asbp_parent_resource (cast `/Game/WorldObjects/Items/ResourceItems/BP_ParentResource` OtherActor))
  (if (and (`self.PlacedDown?`) (`self.Water?`))
    (bind _asbp_uncut_emerald (cast `/Game/WorldObjects/Items/ResourceItems/BP_UncutEmerald` _asbp_parent_resource)
      (:`then`
        (bind _returnvalue_2 (`|SpawnActorFromClass` "/Game/WorldObjects/Items/ResourceItems/BP_Emerald.BP_Emerald_C" (`self.GetTransform` _asbp_uncut_emerald) "Undefined" "OverrideRootScale" null (* (`/Game/WorldObjects/Items/ResourceItems/BP_ParentResource.Size` _asbp_uncut_emerald) _returnvalue) 0 false false true false false "" "" 0 "(INVALID)" null))
        (`self.K2_DestroyActor` _asbp_uncut_emerald)
        (`/Game/WorldObjects/Items/BP_ParentItem.ItemDropped` _returnvalue_2))
      (:`CastFailed`
        (bind _asbp_uncut_ruby (cast `/Game/WorldObjects/Items/ResourceItems/BP_UncutRuby` _asbp_parent_resource)
          (:`then`
            (bind _returnvalue_3 (`|SpawnActorFromClass` "/Game/WorldObjects/Items/ResourceItems/BP_Ruby.BP_Ruby_C" (`self.GetTransform` _asbp_uncut_ruby) "Undefined" "OverrideRootScale" null (* _returnvalue (`/Game/WorldObjects/Items/ResourceItems/BP_ParentResource.Size` _asbp_uncut_ruby)) 0 false false true false false "" "" 0 "(INVALID)" null))
            (`self.K2_DestroyActor` _asbp_uncut_ruby)
            (`/Game/WorldObjects/Items/BP_ParentItem.ItemDropped` _returnvalue_3))
          (:`CastFailed`
            (bind _asbp_uncut_sapphire (cast `/Game/WorldObjects/Items/ResourceItems/BP_UncutSapphire` _asbp_parent_resource))
            (bind _returnvalue_4 (`|SpawnActorFromClass` "/Game/WorldObjects/Items/ResourceItems/BP_Sapphire.BP_Sapphire_C" (`self.GetTransform` _asbp_uncut_sapphire) "Undefined" "OverrideRootScale" null (* (`/Game/WorldObjects/Items/ResourceItems/BP_ParentResource.Size` _asbp_uncut_sapphire) _returnvalue) 0 false false true false false "" "" 0 "(INVALID)" null))
            (`self.K2_DestroyActor` _asbp_uncut_sapphire)
            (`/Game/WorldObjects/Items/BP_ParentItem.ItemDropped` _returnvalue_4)))))))

(fn `UserConstructionScript`
  (`parent.UserConstructionScript`)
  (set `self.ExtraMeshes` (`|MakeArray` (`self.WheelTwo`) (`self.WheelOne`))))