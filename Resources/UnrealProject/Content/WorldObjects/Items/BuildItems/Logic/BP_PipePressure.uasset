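; A buildable pipe pressure booster that burns crystals and shard bars to add pressure to water passing through it.
; A capsule overlap tracks loaded shards; each water input destroys depleted ones, shrinks the first, displays usable content and forwards boosted pressure, or unchanged pressure when empty.
; Clicking swings the door on timelines to toggle the Up state, without which water is not forwarded.
; Signals relay between the two boxes regardless of door state.
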(event `self.SignalIn`
  (params (Box :type String) (Active :type Boolean))
  (switch `string` Box
    (:`Box1`
      (`self.SendSignal` (`self.Box2`) Active))
    (:`Box2`
      (`self.SendSignal` (`self.Box1`) Active))))

(event `self.WaterIn`
  (params (Box :type String) (WaterQuality :type Integer) (WaterPressure :type "Float (single-precision)"))
  (bind _shardarray (`self.ShardArray`))
  (bind _asbp_parent_resource (cast `/Game/WorldObjects/Items/ResourceItems/BP_ParentResource` (`|GetArrayItem` _shardarray) :!pure true))
  (if (`self.Up`)
    (set `self.ContentSize` 0.0)
    (for _array_element _shardarray
      (bind _asbp_parent_resource_2 (cast `/Game/WorldObjects/Items/ResourceItems/BP_ParentResource` _array_element :!pure true))
      (bind _size (`/Game/WorldObjects/Items/ResourceItems/BP_ParentResource.Size` _asbp_parent_resource_2))
      (if (<= _size 0.3)
        (`self.K2_DestroyActor` _asbp_parent_resource_2)
        (else
          (set `self.ContentSize` (+ (`self.ContentSize`) (- _size 0.3))))))
    (if (> (`KismetArrayLibrary.Array_Length` _shardarray) 0)
      (set `/Game/WorldObjects/Items/ResourceItems/BP_ParentResource.Size` (- (`/Game/WorldObjects/Items/ResourceItems/BP_ParentResource.Size` _asbp_parent_resource) 0.005) _asbp_parent_resource)
      (`TextRenderComponent.K2_SetText` (`self.TextRender_0`) (`KismetTextLibrary.Conv_DoubleToText` (`self.ContentSize`) "HalfToEven"))
      (`parent.WaterSwap` Box WaterQuality (+ WaterPressure 25.0))
      (else
        (`parent.WaterSwap` Box WaterQuality WaterPressure)))))

(event `self.OverrideMouseActivated`
  (params (Component :type "ActorComponent Object Reference"))
  (bind _door (`self.Door`))
  (if (`self.Up`)
    (`SceneComponent.K2_SetRelativeRotation` :`self` _door)
    (bind (_direction _newtrack_2) (`Timeline|GoDown` :!via `PlayFromStart`)
      (:`Update`
        (`SceneComponent.K2_SetRelativeRotation` _door (`KismetMathLibrary.MakeRotator` 0.0 _newtrack_2) false false))
      (:`Finished`
        (set `self.Up` false)))
    (else
      (`SceneComponent.K2_SetRelativeRotation` _door (struct :`Pitch` -90.0) false false)
      (bind (_direction_2 _newtrack_2_2) (`Timeline|GoUp` :!via `PlayFromStart`)
        (:`Update`
          (`SceneComponent.K2_SetRelativeRotation` _door (`KismetMathLibrary.MakeRotator` 0.0 _newtrack_2_2) false false))
        (:`Finished`
          (set `self.Up` true))))))

(event `self.Capsule.OnComponentBeginOverlap`
  (params (OverlappedComponent :type "PrimitiveComponent Object Reference") (OtherActor :type "Actor Object Reference") (OtherComp :type "PrimitiveComponent Object Reference") (OtherBodyIndex :type Integer) (bFromSweep :type Boolean) (SweepResult :type "HitResult Structure (by ref)"))
  (bind _shardarray (`self.ShardArray`))
  (cast `/Game/WorldObjects/Items/ResourceItems/BP_Crystal` OtherActor
    (:`then`
      (`KismetArrayLibrary.Array_Add` _shardarray OtherActor))
    (:`CastFailed`
      (cast `/Game/WorldObjects/Items/ResourceItems/BP_ShardBar` OtherActor)
      (`KismetArrayLibrary.Array_Add` _shardarray OtherActor))))

(event `self.Capsule.OnComponentEndOverlap`
  (params (OverlappedComponent :type "PrimitiveComponent Object Reference") (OtherActor :type "Actor Object Reference") (OtherComp :type "PrimitiveComponent Object Reference") (OtherBodyIndex :type Integer))
  (bind _shardarray (`self.ShardArray`))
  (cast `/Game/WorldObjects/Items/ResourceItems/BP_Crystal` OtherActor
    (:`then`
      (`KismetArrayLibrary.Array_RemoveItem` _shardarray OtherActor))
    (:`CastFailed`
      (cast `/Game/WorldObjects/Items/ResourceItems/BP_ShardBar` OtherActor)
      (`KismetArrayLibrary.Array_RemoveItem` _shardarray OtherActor))))

(fn `UserConstructionScript`
  (`parent.UserConstructionScript`)
  (`KismetArrayLibrary.Array_Add` (`self.ExtraMeshes`) (`self.Door`)))