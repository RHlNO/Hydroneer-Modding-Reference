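; BP_PipeXNOR is a buildable XNOR logic gate that outputs on Box 3 when both or neither of its two inputs are active.
; Once placed, an active signal on Box 1 or 2 sets that input and starts a 0.15-second timer to clear it, so inputs persist only while refreshed.
; Every received signal or timeout recounts inputs and sends the result.
; Water input is handed to the parent class.
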(event `Box1Off`
  (bind _totalin (`self.TotalIn`))
  (`KismetArrayLibrary.Array_Set` (`self.Inputs`))
  (`self.CountInputs` :!label _label)
  (`self.SendSignal` (`self.Box3`) (or (== _totalin 0) (== _totalin 2))))

(event `self.SignalIn`
  (params (Box :type String) (Active :type Boolean))
  (bind _inputs (`self.Inputs`))
  (if (`self.PlacedDown?`)
    (switch `string` Box
      (:`Box1`
        (if Active
          (`KismetArrayLibrary.Array_Set` _inputs 0 true)
          (`KismetSystemLibrary.K2_SetTimerDelegate` (delegate `Box1Off`) 0.15)
          (goto _label)
          (else
            (goto _label))))
      (:`Box2`
        (if Active
          (`KismetArrayLibrary.Array_Set` _inputs 1 true)
          (`KismetSystemLibrary.K2_SetTimerDelegate` (delegate `Box2Off`) 0.15)
          (goto _label)
          (else
            (goto _label)))))))

(event `self.WaterIn`
  (params (Box :type String) (WaterQuality :type Integer) (WaterPressure :type "Float (single-precision)"))
  (`parent.WaterIn` Box WaterQuality WaterPressure))

(event `Box2Off`
  (`KismetArrayLibrary.Array_Set` (`self.Inputs`) 1)
  (goto _label))

(fn `UserConstructionScript`
  (`parent.UserConstructionScript`))