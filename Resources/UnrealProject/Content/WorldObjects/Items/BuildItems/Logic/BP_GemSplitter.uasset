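; Water-powered buildable that sorts Emerald, Ruby and Sapphire items into three directional output lanes, sending other items to the middle lane.
; Water into Box1 powers it for 1.5 seconds and is traced onward from each box at reduced pressure, spilling as projectiles where unconnected and uncorked.
; While powered, overlapping items are stopped and teleported out along their lane.
; Left and right buttons swap neighboring lane assignments and reposition the gem indicators.
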(event `NoWater`
  (set `self.Water?` false))

(event `self.WaterIn`
  (params (Box :type String) (WaterQuality :type Integer) (WaterPressure :type "Float (single-precision)"))
  (if (and (`self.PlacedDown?`) (`KismetStringLibrary.EqualEqual_StrStr` Box "Box1"))
    (set `self.Water?` true)
    (`KismetSystemLibrary.K2_SetTimerDelegate` (delegate `NoWater`) 1.5)
    (for _array_element (`self.Boxes`)
      (bind (_returnvalue_x _returnvalue_y _returnvalue_z) (`KismetMathLibrary.BreakVector` (`SceneComponent.K2_GetComponentLocation` _array_element)))
      (bind _outhit (`KismetSystemLibrary.LineTraceSingle` (`KismetMathLibrary.MakeVector` (- _returnvalue_x 2.0) (- _returnvalue_y 2.0) (- _returnvalue_z 2.0)) (`KismetMathLibrary.MakeVector` (+ _returnvalue_x 2.0) (+ _returnvalue_y 2.0) (+ _returnvalue_z 2.0)) "TraceTypeQuery1" true))
      (bind (_bblockinghit _binitialoverlap _time _distance _location _impactpoint _normal _impactnormal _physmat _hitactor _hitcomponent) (`GameplayStatics.BreakHitResult` _outhit))
      (if (not (`KismetStringLibrary.EqualEqual_StrStr` (`KismetSystemLibrary.GetClassDisplayName` (`GameplayStatics.GetObjectClass` _hitactor)) "BP_PipeCork_C"))
        (bind _asbp_parent_water_item (cast `/Game/WorldObjects/Items/BuildItems/BP_ParentWaterItem` _hitactor)
          (:`then`
            (`self.WaterIn` _asbp_parent_water_item (`KismetSystemLibrary.GetObjectName` _hitcomponent) (`KismetMathLibrary.Clamp` WaterQuality 1 10) (`KismetMathLibrary.FClamp` (- WaterPressure 1.0) 1.0 100.0)))
          (:`CastFailed`
            (`|SpawnActorFromClass` "/Game/WorldObjects/BP_ProjectileWater.BP_ProjectileWater_C" (`SceneComponent.K2_GetComponentToWorld` _array_element) "Undefined" "OverrideRootScale" null null)))))))

(event `self.Box.OnComponentBeginOverlap`
  (params (OverlappedComponent :type "PrimitiveComponent Object Reference") (OtherActor :type "Actor Object Reference") (OtherComp :type "PrimitiveComponent Object Reference") (OtherBodyIndex :type Integer) (bFromSweep :type Boolean) (SweepResult :type "HitResult Structure (by ref)"))
  (if (`self.Water?`)
    (bind _asbp_parent_item (cast `/Game/WorldObjects/Items/BP_ParentItem` OtherActor))
    (bind _asbp_emerald (cast `/Game/WorldObjects/Items/ResourceItems/BP_Emerald` OtherActor)
      (:`then`
        (`self.OutPut` _asbp_emerald (`KismetArrayLibrary.Array_Find` (`self.Lanes`) "Emerald")))
      (:`CastFailed`
        (bind _asbp_ruby (cast `/Game/WorldObjects/Items/ResourceItems/BP_Ruby` OtherActor)
          (:`then`
            (`self.OutPut` _asbp_ruby (`KismetArrayLibrary.Array_Find` (`self.Lanes`) "Ruby")))
          (:`CastFailed`
            (bind _asbp_sapphire (cast `/Game/WorldObjects/Items/ResourceItems/BP_Sapphire` OtherActor)
              (:`then`
                (`self.OutPut` _asbp_sapphire (`KismetArrayLibrary.Array_Find` (`self.Lanes`) "Sapphire")))
              (:`CastFailed`
                (`self.OutPut` _asbp_parent_item 1)))))))))

(event `self.OverrideMouseActivated`
  (params (Component :type "ActorComponent Object Reference"))
  (bind _lanes (`self.Lanes`))
  (bind _buttons (`self.Buttons`))
  (bind _lanes_2 (`self.Lanes`))
  (bind _buttons_2 (`self.Buttons`))
  (switch `string` (`KismetSystemLibrary.GetObjectName` Component)
    (:`ButtonLeft`
      (set `self.Lanes` (`|MakeArray` (`|GetArrayItem` _lanes_2 1) (`|GetArrayItem` _lanes_2) (`|GetArrayItem` _lanes_2 2)))
      (set `self.Buttons` (`|MakeArray` (`|GetArrayItem` _buttons_2 1) (`|GetArrayItem` _buttons_2) (`|GetArrayItem` _buttons_2 2))))
    (:`ButtonRight`
      (set `self.Lanes` (`|MakeArray` (`|GetArrayItem` _lanes) (`|GetArrayItem` _lanes 2) (`|GetArrayItem` _lanes 1)))
      (set `self.Buttons` (`|MakeArray` (`|GetArrayItem` _buttons) (`|GetArrayItem` _buttons 2) (`|GetArrayItem` _buttons 1)))))
  (`self.SetButtons`))

(fn `OutPut`
  (params (Item :type "/Game/WorldObjects/Items/BP_ParentItem Object Reference") (Lane :type Integer))
  (bind _returnvalue (`self.GetTransform`))
  (`PrimitiveComponent.SetAllPhysicsLinearVelocity` (`/Game/WorldObjects/Items/BP_ParentItem.StaticMesh` Item) (0.0 0.0 0.0) false)
  (`self.K2_SetActorLocation` Item (`KismetMathLibrary.MakeVector` (.x (.location _returnvalue)) (.y (.location _returnvalue)) (+ (.z (.location _returnvalue)) 35.0)) false true)
  (switch `int` Lane
    (:`0`
      (`self.K2_SetActorRotation` Item (`KismetMathLibrary.MakeRotator` 0.0 0.0 (- (.yaw (.rotation _returnvalue)) 180.0)) true))
    (:`1`
      (`self.K2_SetActorRotation` Item (`KismetMathLibrary.MakeRotator` 0.0 0.0 (- (.yaw (.rotation _returnvalue)) 90.0)) true))
    (:`2`
      (`self.K2_SetActorRotation` Item (`KismetMathLibrary.MakeRotator` 0.0 0.0 (.yaw (.rotation _returnvalue))) true)))
  (`self.K2_SetActorLocation` Item (+ (`self.K2_GetActorLocation` Item) (* (`self.GetActorForwardVector` Item) 50.0)) false true)
  (`self.ItemDropped` Item))

(fn `SetButtons`
  (bind _buttons (`self.Buttons`))
  (`SceneComponent.K2_SetRelativeLocation` (`|GetArrayItem` _buttons) (-15.0 48.0 117.0) false false)
  (`SceneComponent.K2_SetRelativeLocation` (`|GetArrayItem` _buttons 1) (0.0 48.0 117.0) false false)
  (`SceneComponent.K2_SetRelativeLocation` (`|GetArrayItem` _buttons 2) (15.0 48.0 117.0) false false))

(fn `UserConstructionScript`
  (bind _buttonruby (`self.ButtonRuby`))
  (bind _buttonsapphire (`self.ButtonSapphire`))
  (bind _buttonemerald (`self.ButtonEmerald`))
  (`parent.UserConstructionScript`)
  (set `self.ExtraMeshes` (`|MakeArray` _buttonruby _buttonsapphire _buttonemerald (`self.Screens`) (`self.ButtonRight`) (`self.ButtonLeft`)))
  (set `self.Buttons` (`|MakeArray` _buttonemerald _buttonruby _buttonsapphire)))