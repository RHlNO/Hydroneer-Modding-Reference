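; BP_PipeReader is a buildable inline pipe gauge that displays the quality and pressure of water passing through it.
; Incoming water rotates a mesh by pressure through a clamped range mapping, updates two text renders, and is handed to the parent's WaterSwap.
; Signals received on either of its two boxes are relayed out of the opposite one.
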(event `self.SignalIn`
  (params (Box :type String) (Active :type Boolean))
  (switch `string` Box
    (:`Box1`
      (`self.SendSignal` (`self.Box2`) Active))
    (:`Box2`
      (`self.SendSignal` (`self.Box1`) Active))))

(event `self.WaterIn`
  (params (Box :type String) (WaterQuality :type Integer) (WaterPressure :type "Float (single-precision)"))
  (`SceneComponent.K2_SetRelativeRotation` (`self.StaticMesh2`) (`KismetMathLibrary.MakeRotator` 0.0 0.0 (`KismetMathLibrary.MapRangeClamped` WaterPressure 1.0 100.0 0.0 180.0)) false false)
  (`parent.WaterSwap` Box WaterQuality WaterPressure)
  (`TextRenderComponent.K2_SetText` (`self.TextRender5`) (`KismetTextLibrary.Conv_IntToText` WaterQuality))
  (`TextRenderComponent.K2_SetText` (`self.TextRender6`) (`KismetTextLibrary.Conv_DoubleToText` WaterPressure "HalfToEven")))

(fn `UserConstructionScript`
  (`parent.UserConstructionScript`))