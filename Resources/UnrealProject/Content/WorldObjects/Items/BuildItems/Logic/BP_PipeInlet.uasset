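; BP_PipeInlet is a buildable pipe inlet that feeds water into the pipe system while placed in water.
; Its construction script starts looping timers for GenerateWater and GenerateSignal.
; GenerateWater sends fixed-quality, pressurized water through Box2 and plays a timeline pulse that slides two indicators.
; A parallel WaterGenerate event does the same while also starting or stopping the attached intake sound.
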(event `WaterGenerate`
  (bind _intakenoise (`self.IntakeNoise`))
  (if (and (`self.InWater?`) (`self.PlacedDown?`))
    (if (not (`KismetSystemLibrary.IsValid` (`self.IntakeNoise`)))
      (bind _returnvalue (`GameplayStatics.SpawnSoundAttached` "/Game/Sound/Construction/Water_Inlet.Water_Inlet" (`self.Box_0`) "None" (0.0 0.0 0.0) (struct) "KeepRelativeOffset" true 0.7 1.0 0.0 "/Game/Sound/EnvLoops/SA_SmallEnv.SA_SmallEnv" null))
      (set `self.IntakeNoise` _returnvalue))
    (`self.PulseWater`)
    (`self.SendWater` (`self.Box2`) 1 50.0)
    (elif (`KismetSystemLibrary.IsValid` _intakenoise)
      (`AudioComponent.Stop` _intakenoise))))

(event `PulseWater`
  (bind _indicator2 (`self.Indicator2`))
  (bind (_direction _newtrack_0) (`Timeline|Timeline_1` :!via `PlayFromStart`)
    (:`Update`
      (`SceneComponent.SetVisibility` _indicator2 true false)
      (`SceneComponent.K2_SetRelativeLocation` (`self.Indicator3`) (`KismetMathLibrary.MakeVector` _newtrack_0 0.0 121.0) false false)
      (`SceneComponent.K2_SetRelativeLocation` _indicator2 (`KismetMathLibrary.MakeVector` (- _newtrack_0 33.330002) 0.0 121.0) false false)
      (if (and (`SceneComponent.IsVisible` _indicator2) (> _newtrack_0 56.0))
        (`SceneComponent.SetVisibility` _indicator2 false false)))))

(event `self.OverrideMouseActivated`
  (params (Component :type "ActorComponent Object Reference"))
  (`/Game/BP_GameController.ReturnNoActivation` (cast `/Game/BP_GameController` (`GameplayStatics.GetPlayerController` 0) :!pure true) (`ActorComponent.GetOwner` Component)))

(fn `GenerateWater`
  (if (and (`self.InWater?`) (`self.PlacedDown?`))
    (`self.PulseWater`)
    (`self.SendWater` (`self.Box2`) 1 50.0)))

(fn `UserConstructionScript`
  (`parent.UserConstructionScript`)
  (`KismetSystemLibrary.K2_SetTimer` null "GenerateWater" (`self.WaterTimer`) true)
  (`KismetSystemLibrary.K2_SetTimer` null "GenerateSignal" (`self.SignalTimer`) true))