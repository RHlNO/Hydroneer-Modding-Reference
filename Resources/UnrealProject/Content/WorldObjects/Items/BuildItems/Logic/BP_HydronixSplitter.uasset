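; Placeable Hydronix splitter that, while powered by incoming water, sorts overlapping items into left, forward or right lanes by class.
; Water entering Box1 starts a timed active window and is traced onward from each box to connected water items at reduced pressure, or sprayed as projectiles unless corked.
; Screen buttons cycle resource types and set each lane in the Sortables map, highlighted by arrows.
; OutPut teleports and launches items; unmapped non-resources go forward.
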(event `NoWater`
  (set `self.Water?` false))

(event `self.WaterIn`
  (params (Box :type String) (WaterQuality :type Integer) (WaterPressure :type "Float (single-precision)"))
  (if (and (`self.PlacedDown?`) (`KismetStringLibrary.EqualEqual_StrStr` Box "Box1"))
    (set `self.Water?` true)
    (`KismetSystemLibrary.K2_SetTimerDelegate` (delegate `NoWater`) 1.5)
    (for _array_element (`self.Boxes`)
      (bind (_returnvalue_x _returnvalue_y _returnvalue_z) (`KismetMathLibrary.BreakVector` (`SceneComponent.K2_GetComponentLocation` _array_element)))
      (bind _outhit (`KismetSystemLibrary.LineTraceSingle` (`KismetMathLibrary.MakeVector` (- _returnvalue_x 2.0) (- _returnvalue_y 2.0) (- _returnvalue_z 2.0)) (`KismetMathLibrary.MakeVector` (+ _returnvalue_x 2.0) (+ _returnvalue_y 2.0) (+ _returnvalue_z 2.0)) "TraceTypeQuery1" true))
      (bind (_bblockinghit _binitialoverlap _time _distance _location _impactpoint _normal _impactnormal _physmat _hitactor _hitcomponent) (`GameplayStatics.BreakHitResult` _outhit))
      (if (not (`KismetStringLibrary.EqualEqual_StrStr` (`KismetSystemLibrary.GetClassDisplayName` (`GameplayStatics.GetObjectClass` _hitactor)) "BP_PipeCork_C"))
        (bind _asbp_parent_water_item (cast `/Game/WorldObjects/Items/BuildItems/BP_ParentWaterItem` _hitactor)
          (:`then`
            (`self.WaterIn` _asbp_parent_water_item (`KismetSystemLibrary.GetObjectName` _hitcomponent) (`KismetMathLibrary.Clamp` WaterQuality 1 10) (`KismetMathLibrary.FClamp` (- WaterPressure 1.0) 1.0 100.0)))
          (:`CastFailed`
            (`|SpawnActorFromClass` "/Game/WorldObjects/BP_ProjectileWater.BP_ProjectileWater_C" (`SceneComponent.K2_GetComponentToWorld` _array_element) "Undefined" "OverrideRootScale" null null)))))))

(event `self.Box.OnComponentBeginOverlap`
  (params (OverlappedComponent :type "PrimitiveComponent Object Reference") (OtherActor :type "Actor Object Reference") (OtherComp :type "PrimitiveComponent Object Reference") (OtherBodyIndex :type Integer) (bFromSweep :type Boolean) (SweepResult :type "HitResult Structure (by ref)"))
  (if (`self.Water?`)
    (bind _asbp_parent_item (cast `/Game/WorldObjects/Items/BP_ParentItem` OtherActor))
    (bind _asbp_parent_resource (cast `/Game/WorldObjects/Items/ResourceItems/BP_ParentResource` _asbp_parent_item)
      (:`then`
        (switch `int` (`BlueprintMapLibrary.Map_Find` (`self.Sortables`) (`GameplayStatics.GetObjectClass` _asbp_parent_item))
          (:`Default`
            (`self.OutPut` _asbp_parent_item 1 :!label _label))
          (:`0`
            (`self.OutPut` _asbp_parent_resource))
          (:`1`
            (`self.OutPut` _asbp_parent_resource 1))
          (:`2`
            (`self.OutPut` _asbp_parent_resource 2))))
      (:`CastFailed`
        (goto _label)))))

(event `self.OverrideMouseActivated`
  (params (Component :type "ActorComponent Object Reference"))
  (bind _sortablelist (`self.SortableList`))
  (bind _screenindex (`self.ScreenIndex`))
  (bind _sortables (`self.Sortables`))
  (bind _returnvalue (`KismetArrayLibrary.Array_Length` _sortablelist))
  (bind _output (`|GetArrayItem` _sortablelist (`self.ScreenIndex`)))
  (bind _output_2 (`|GetArrayItem` (`self.SortableList`) (`self.ScreenIndex`)))
  (switch `string` (`KismetSystemLibrary.GetObjectName` Component)
    (:`Default`
      _)
    (:`TxtLeft`
      (bind _result (`/Engine/EditorBlueprintResources/StandardMacros.DecrementInt` _screenindex)
        (:`  `
          (if (< _result 0)
            (set `self.ScreenIndex` (- _returnvalue 1)))
          (`TextRenderComponent.K2_SetText` (`self.TextRender`) (`.Name` (defaults `/Game/WorldObjects/Items/BuildItems/Logic/BP_HydronixSplitter` _output)) :!label _label_2)
          (`self.LightButton` (`BlueprintMapLibrary.Map_Find` (`self.Sortables`) _output)))))
    (:`TxtRight`
      (bind _result_2 (`/Engine/EditorBlueprintResources/StandardMacros.IncrementInt` _screenindex)
        (:`  `
          (if (>= _result_2 _returnvalue)
            (set `self.ScreenIndex` 0)
            (goto _label_2)
            (else
              (goto _label_2))))))
    (:`Left`
      (`BlueprintMapLibrary.Map_Add` _sortables _output_2)
      (`self.LightButton` 0))
    (:`Right`
      (`BlueprintMapLibrary.Map_Add` _sortables _output_2 2)
      (`self.LightButton` 2))
    (:`Forward`
      (`BlueprintMapLibrary.Map_Add` _sortables _output_2 1)
      (`self.LightButton` 1)))
  (`/Game/BP_GameController.ReturnNoActivation` (cast `/Game/BP_GameController` (`GameplayStatics.GetPlayerController` 0) :!pure true) (`ActorComponent.GetOwner` Component)))

(event `self.ReceiveBeginPlay`
  (if (`self.PlacedDown?`)
    (`SceneComponent.SetWorldScale3D` (`self.StaticMesh`) (1.0 1.0 1.0)))
  (`parent.ReceiveBeginPlay`))

(event `self.OverrideClickNoTarget`
  (params (Controller :type "/Game/BP_GameController Object Reference") (`Hit Actor` :type "Actor Object Reference"))
  (`SceneComponent.SetWorldScale3D` (`self.StaticMesh`) (1.0 1.0 1.0))
  (`parent.OverrideClickNoTarget` Controller `Hit Actor`))

(event `self.OverrideRightClickNoTarget`
  (bind _asbp_game_controller (cast `/Game/BP_GameController` (`GameplayStatics.GetPlayerController` 0) :!pure true))
  (bind _truedrop (`/Game/BP_GameController.DropItem` _asbp_game_controller))
  (if _truedrop
    (`SceneComponent.SetWorldScale3D` (`self.StaticMesh`) (0.2 0.2 0.2))
    (`/Game/BP_GameController.PickUpItem` _asbp_game_controller self)))

(event `self.OverrideDroppedItem`
  (`SceneComponent.SetWorldScale3D` (`self.StaticMesh`) (0.2 0.2 0.2))
  (`parent.OverrideDroppedItem`))

(event `self.OverridePickedup`
  (`SceneComponent.SetWorldScale3D` (`self.StaticMesh`) (0.2 0.2 0.2))
  (`parent.OverridePickedup`))

(fn `LightButton`
  (params (Direction :type Integer))
  (locals (LightUp :type "ArrowComponent Object Reference"))
  (bind _arrow3 (`self.Arrow3`))
  (bind _arrow4 (`self.Arrow4`))
  (bind _arrow (`self.Arrow`))
  (switch `int` Direction
    (:`0`
      (set `local.LightUp` _arrow3))
    (:`1`
      (set `local.LightUp` _arrow4))
    (:`2`
      (set `local.LightUp` _arrow)))
  (`ArrowComponent.SetArrowColor` _arrow3 (struct :`R` 1.0 :`A` 1.0))
  (`ArrowComponent.SetArrowColor` _arrow4 (struct :`R` 1.0 :`A` 1.0))
  (`ArrowComponent.SetArrowColor` _arrow (struct :`R` 1.0 :`A` 1.0))
  (`ArrowComponent.SetArrowColor` (`local.LightUp`) (struct :`G` 1.0 :`A` 1.0)))

(fn `OutPut`
  (params (Item :type "/Game/WorldObjects/Items/BP_ParentItem Object Reference") (Lane :type Integer))
  (bind _returnvalue (`self.GetTransform`))
  (bind _staticmesh (`/Game/WorldObjects/Items/BP_ParentItem.StaticMesh` Item))
  (bind _returnvalue_2 (* (`self.GetActorForwardVector` Item) 50.0))
  (`PrimitiveComponent.SetAllPhysicsLinearVelocity` _staticmesh (0.0 0.0 0.0) false)
  (`self.K2_SetActorLocation` Item (`KismetMathLibrary.MakeVector` (.x (.location _returnvalue)) (.y (.location _returnvalue)) (+ (.z (.location _returnvalue)) 50.0)) false true)
  (switch `int` Lane
    (:`0`
      (`self.K2_SetActorRotation` Item (`KismetMathLibrary.MakeRotator` 0.0 0.0 (- (.yaw (.rotation _returnvalue)) 180.0)) true))
    (:`1`
      (`self.K2_SetActorRotation` Item (`KismetMathLibrary.MakeRotator` 0.0 0.0 (- (.yaw (.rotation _returnvalue)) 90.0)) true))
    (:`2`
      (`self.K2_SetActorRotation` Item (`KismetMathLibrary.MakeRotator` 0.0 0.0 (.yaw (.rotation _returnvalue))) true)))
  (`self.K2_SetActorLocation` Item (+ (`self.K2_GetActorLocation` Item) _returnvalue_2) false true)
  (`PrimitiveComponent.AddImpulse` _staticmesh (* _returnvalue_2 2) "None" true))

(fn `UserConstructionScript`
  (`parent.UserConstructionScript`)
  (set `self.ExtraMeshes` (`|MakeArray` (`self.Screens`)))
  (bind _keys (`BlueprintMapLibrary.Map_Keys` (`self.Sortables`)))
  (set `self.SortableList` _keys))