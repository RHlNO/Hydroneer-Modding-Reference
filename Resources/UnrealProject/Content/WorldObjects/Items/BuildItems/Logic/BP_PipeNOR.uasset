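; BP_PipeNOR is a buildable logic pipe item that acts as a NOR gate.
; Incoming signals update the inherited input total, and it sends a signal on Box3 that is true only when that total is not above zero.
; Incoming water is forwarded to the shared water-in logic, and mouse activation is overridden to return no click.
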(event `self.SignalIn`
  (params (NewParam :type String) (NewParam2 :type Boolean))
  (`self.LogicSignalIn` NewParam NewParam2)
  (`self.SendSignal` (`self.Box3`) (not (> (`self.TotalIn`) 0))))

(event `/Game/WorldObjects/Items/BuildItems/BP_ParentWaterItem.WaterIn`
  (params (Box :type String) (WaterQuality :type Integer) (WaterPressure :type "Float (single-precision)"))
  (`self.LogicWaterIn` WaterQuality WaterPressure))

(event `/Game/WorldObjects/Items/BP_ParentItem.OverrideMouseActivated`
  (params (Component :type "ActorComponent Object Reference"))
  (`self.ReturnNoClick` null))

(fn `UserConstructionScript`
  (`parent.UserConstructionScript`))