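; BP_PipeDelay is a buildable pipe item that delays signals between its two boxes and hands incoming water to WaterSwap.
; Incoming values queue in History; once the count exceeds Delay, the oldest goes out the opposite box, so delay counts signal events.
; Each output restarts a short timer that clears History when it fires.
; Mouse activation cycles Delay, clears the queue and shows Delay as tenths on a text render.
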(event `CustomEvent_0`
  (`KismetArrayLibrary.Array_Clear` (`self.History`)))

(event `self.SignalIn`
  (params (NewParam :type String) (NewParam2 :type Boolean))
  (bind _history (`self.History`))
  (bind _history_2 (`self.History`))
  (bind _signaltemp (`self.SignalTemp`))
  (`KismetArrayLibrary.Array_Add` _history NewParam2)
  (if (> (`KismetArrayLibrary.Array_Length` _history) (`self.Delay`))
    (set `self.SignalTemp` (`|GetArrayItem` _history_2))
    (`KismetArrayLibrary.Array_Remove` _history_2)
    (`KismetSystemLibrary.K2_SetTimerDelegate` (delegate `CustomEvent_0`) 0.15)
    (switch `string` NewParam
      (:`Box1`
        (`self.SendSignal` (`self.Box2`) _signaltemp))
      (:`Box2`
        (`self.SendSignal` (`self.Box1`) _signaltemp)))))

(event `self.WaterIn`
  (params (Box :type String) (WaterQuality :type Integer) (WaterPressure :type "Float (single-precision)"))
  (`self.WaterSwap` Box WaterQuality WaterPressure))

(event `/Game/WorldObjects/Items/BP_ParentItem.OverrideMouseActivated`
  (params (Component :type "ActorComponent Object Reference"))
  (bind _output_get (set `self.Delay` (+ (`self.Delay`) 1)))
  (if (> _output_get 10)
    (set `self.Delay` 0))
  (`KismetArrayLibrary.Array_Clear` (`self.History`))
  (`self.UpdateText`))

(event `UpdateText`
  (`TextRenderComponent.K2_SetText` (`self.TextRender5`) (`KismetTextLibrary.Conv_DoubleToText` (/ (`KismetMathLibrary.Conv_IntToDouble` (`self.Delay`)) 10.0) "HalfToEven")))

(fn `UserConstructionScript`
  (`parent.UserConstructionScript`))