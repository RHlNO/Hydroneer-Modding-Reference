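; BP_GemCrusher is a placeable, water-powered machine that destroys resource actors hitting either of its cylinders.
; Incoming water wears down Durability by an amount based on water quality, starts the timeline-driven blade rotation and keeps the crusher active until a short timer clears it.
; Each crushed resource briefly speeds up the blades; no output is spawned here.
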(event `SpinBlades`
  (bind _bladespeed (`self.BladeSpeed`))
  ;[1 1 1] Rotation of Blades
  (`Timeline|Timeline_0_0` :!via `PlayFromStart`
    (:`Update`
      (`SceneComponent.K2_AddLocalRotation` (`self.StaticMesh1`) (`KismetMathLibrary.MakeRotator` 0.0 _bladespeed) false false)
      (`SceneComponent.K2_AddLocalRotation` (`self.StaticMesh4`) (`KismetMathLibrary.MakeRotator` 0.0 _bladespeed) false false)
      (`SceneComponent.K2_AddLocalRotation` (`self.StaticMesh2`) (`KismetMathLibrary.MakeRotator` 0.0 _bladespeed) false false)
      (`SceneComponent.K2_AddLocalRotation` (`self.StaticMesh5`) (`KismetMathLibrary.MakeRotator` 0.0 _bladespeed) false false)
      (`SceneComponent.K2_AddLocalRotation` (`self.StaticMesh3`) (`KismetMathLibrary.MakeRotator` 0.0 _bladespeed) false false)
      (`SceneComponent.K2_AddLocalRotation` (`self.StaticMesh6`) (`KismetMathLibrary.MakeRotator` 0.0 _bladespeed) false false)
      (`SceneComponent.K2_AddLocalRotation` (`self.StaticMesh7`) (`KismetMathLibrary.MakeRotator` 0.0 0.0 (* _bladespeed 4.0)) false false))))

(event `self.ToggleWires`
  (params (Visible :type Boolean))
  (`parent.ToggleWires` false))

(event `WaterGone`
  (set `self.Water?` false))

(event `/Game/WorldObjects/Items/BuildItems/BP_ParentWaterItem.WaterIn`
  (params (Box :type String) (WaterQuality :type Integer) (WaterPressure :type "Float (single-precision)"))
  (if (> (`self.Durability`) 0.0)
    (set `self.Durability` (- (`self.Durability`) (`KismetMathLibrary.Conv_IntToDouble` (* (/ (- 10 WaterQuality) 100) 2))))
    (`self.SpinBlades`)
    (set `self.Water?` true)
    (`KismetSystemLibrary.K2_SetTimerDelegate` (delegate `WaterGone`) 1.5)))

(event `self.Cylinder1.OnComponentHit`
  (params (HitComponent :type "PrimitiveComponent Object Reference") (OtherActor :type "Actor Object Reference") (OtherComp :type "PrimitiveComponent Object Reference") (NormalImpulse :type "Vector Structure") (Hit :type "HitResult Structure (by ref)"))
  (bind _newvar_0_0 (`self.NewVar_0_0`))
  (set `self.NewVar_0_0` OtherActor)
  (if (and (`self.PlacedDown?`) (`self.Water?`)) :!label _label
    (cast `/Game/WorldObjects/Items/ResourceItems/BP_ParentResource` _newvar_0_0)
    (set `self.BladeSpeed` 3.0)
    (`KismetSystemLibrary.K2_SetTimerDelegate` (delegate `SlowDown`) 1.0)
    (`self.K2_DestroyActor` _newvar_0_0)))

(event `SlowDown`
  (set `self.BladeSpeed` 1.0))

(event `self.Cylinder2.OnComponentHit`
  (params (HitComponent :type "PrimitiveComponent Object Reference") (OtherActor :type "Actor Object Reference") (OtherComp :type "PrimitiveComponent Object Reference") (NormalImpulse :type "Vector Structure") (Hit :type "HitResult Structure (by ref)"))
  (set `self.NewVar_0_0` OtherActor)
  (goto _label))

(fn `UserConstructionScript`
  (`parent.UserConstructionScript`))