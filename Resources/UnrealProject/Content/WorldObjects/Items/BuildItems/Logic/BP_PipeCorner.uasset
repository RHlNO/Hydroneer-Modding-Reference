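; Corner pipe build item that relays water and on/off signals through its connection boxes.
; Once placed, an incoming signal marks its box, identified by the last character of its name, as an input and starts a short per-input "Off" timer.
; With one or two inputs, it signals the remaining boxes, active when TotalPlus is positive.
; Incoming water passes its quality and pressure to every non-input box.
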(event `/Game/WorldObjects/Items/BuildItems/BP_ParentWaterItem.WaterIn`
  (params (Box :type String) (WaterQuality :type Integer) (WaterPressure :type "Float (single-precision)"))
  (for (_array_element _array_index) (`self.Inputs`)
    (if (not _array_element)
      (`self.SendWater` (`|GetArrayItem` (`self.Boxes`) _array_index) WaterQuality WaterPressure))))

(event `self.SignalIn`
  (params (Box :type String) (Active :type Boolean))
  (bind _lastin (`self.LastIn`))
  (bind _totalin (`self.TotalIn`))
  (if (`self.PlacedDown?`)
    (set `self.LastIn` (- (`KismetStringLibrary.Conv_StringToInt` (`KismetStringLibrary.Right` Box 1)) 1))
    (`KismetArrayLibrary.Array_Set` (`self.Inputs`) _lastin true true)
    (`KismetArrayLibrary.Array_Set` (`self.Flow`) _lastin Active true)
    (`KismetSystemLibrary.K2_SetTimer` null (`KismetStringLibrary.Concat_StrStr` "Off" (`KismetStringLibrary.Conv_IntToString` _lastin)) 0.15)
    (`self.CountInputs`)
    (if (or (== _totalin 1) (== _totalin 2))
      (for (_array_element _array_index) (`self.Inputs`)
        (if (not _array_element)
          (`self.SendSignal` (`|GetArrayItem` (`self.Boxes`) _array_index) (> (`self.TotalPlus`) 0)))))))

(fn `UserConstructionScript`
  (`parent.UserConstructionScript`))