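; BP_PipeBend is a buildable pipe bend item with two connection boxes that carries signals and water.
; A signal arriving at either box is sent out through the other with the same active state.
; Incoming water is handed to the parent's WaterSwap logic with its box, quality and pressure.
; Mouse activation only calls ReturnNoActivation on the game controller, and construction defers to the parent.
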(event `self.SignalIn`
  (params (Box :type String) (Active :type Boolean))
  (switch `string` Box
    (:`Box1`
      (`self.SendSignal` (`self.Box2`) Active))
    (:`Box2`
      (`self.SendSignal` (`self.Box1`) Active))))

(event `self.WaterIn`
  (params (Box :type String) (WaterQuality :type Integer) (WaterPressure :type "Float (single-precision)"))
  (`parent.WaterSwap` Box WaterQuality WaterPressure))

(event `/Game/WorldObjects/Items/BP_ParentItem.OverrideMouseActivated`
  (params (Component :type "ActorComponent Object Reference"))
  (bind _asbp_game_controller (cast `/Game/BP_GameController` (`GameplayStatics.GetPlayerController` 0)))
  (`/Game/BP_GameController.ReturnNoActivation` _asbp_game_controller (`ActorComponent.GetOwner` Component)))

(fn `UserConstructionScript`
  (`parent.UserConstructionScript`))