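; BP_HydronixVault is a buildable-item vault whose sliding doors open after a scanner sequence triggered by capsule overlap.
; The first overlap shows a scanner light and runs a timeline rotating the scanner scene, then shows a point light and calls OpenDoor.
; Separate timelines slide the door panels and braces along X for opening and closing.
; Nothing here calls CloseDoor or resets the Closed flag, and the trailing delay leads nowhere.
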(event `CloseDoor`
  (bind (_direction _leftouter _leftinner _rightouter _rightinner) (`Timeline|Timeline_1` :!via `ReverseFromEnd`)
    (:`Update`
      (`SceneComponent.K2_SetRelativeLocation` (`self.FrontLeftDoor`) (`KismetMathLibrary.MakeVector` _leftouter 24.4 -50.0) false false)
      (`SceneComponent.K2_SetRelativeLocation` (`self.BottomLeftBrace`) (`KismetMathLibrary.MakeVector` _leftouter -2.200001) false false)
      (`SceneComponent.K2_SetRelativeLocation` (`self.TopLeftBrace`) (`KismetMathLibrary.MakeVector` _leftouter -2.200001 83.0) false false)
      (`SceneComponent.K2_SetRelativeLocation` (`self.BackLeftDoor`) (`KismetMathLibrary.MakeVector` _leftinner 0.0 -50.09) false false)
      (`SceneComponent.K2_SetRelativeLocation` (`self.FrontRightDoor`) (`KismetMathLibrary.MakeVector` _rightouter 23.999964 164.0) false false)
      (`SceneComponent.K2_SetRelativeLocation` (`self.BottomRightBrace`) (`KismetMathLibrary.MakeVector` _rightouter -22.200001) false false)
      (`SceneComponent.K2_SetRelativeLocation` (`self.TopRightBrace`) (`KismetMathLibrary.MakeVector` _rightouter -22.200001 83.0) false false)
      (`SceneComponent.K2_SetRelativeLocation` (`self.BackRightDoor`) (`KismetMathLibrary.MakeVector` _rightinner -24.400019 -50.09) false false))))

(event `OpenDoor`
  (bind (_direction _leftouter _leftinner _rightouter _rightinner) (`Timeline|Timeline_0` :!via `PlayFromStart`)
    (:`Update`
      (`SceneComponent.K2_SetRelativeLocation` (`self.FrontLeftDoor`) (`KismetMathLibrary.MakeVector` _leftouter 24.4 -50.0) false false)
      (`SceneComponent.K2_SetRelativeLocation` (`self.BottomLeftBrace`) (`KismetMathLibrary.MakeVector` _leftouter -2.200001) false false)
      (`SceneComponent.K2_SetRelativeLocation` (`self.TopLeftBrace`) (`KismetMathLibrary.MakeVector` _leftouter -2.200001 83.0) false false)
      (`SceneComponent.K2_SetRelativeLocation` (`self.BackLeftDoor`) (`KismetMathLibrary.MakeVector` _leftinner 0.0 -50.09) false false)
      (`SceneComponent.K2_SetRelativeLocation` (`self.FrontRightDoor`) (`KismetMathLibrary.MakeVector` _rightouter 23.999964 164.0) false false)
      (`SceneComponent.K2_SetRelativeLocation` (`self.BottomRightBrace`) (`KismetMathLibrary.MakeVector` _rightouter -22.200001) false false)
      (`SceneComponent.K2_SetRelativeLocation` (`self.TopRightBrace`) (`KismetMathLibrary.MakeVector` _rightouter -22.200001 83.0) false false)
      (`SceneComponent.K2_SetRelativeLocation` (`self.BackRightDoor`) (`KismetMathLibrary.MakeVector` _rightinner -24.400019 -50.09) false false))))

(event `self.Capsule.OnComponentBeginOverlap`
  (params (OverlappedComponent :type "PrimitiveComponent Object Reference") (OtherActor :type "Actor Object Reference") (OtherComp :type "PrimitiveComponent Object Reference") (OtherBodyIndex :type Integer) (bFromSweep :type Boolean) (SweepResult :type "HitResult Structure (by ref)"))
  (bind _scannerlight (`self.ScannerLight`))
  (if (`self.Closed?`)
    (set `self.Closed?` false)
    (`SceneComponent.SetVisibility` _scannerlight true false)
    (bind (_direction _newtrack_0) (`Timeline|Timeline` :!via `PlayFromStart`)
      (:`Update`
        (`SceneComponent.K2_SetRelativeRotation` (`self.Scene`) (`KismetMathLibrary.MakeRotator` 0.0 _newtrack_0 -269.999176) false false))
      (:`Finished`
        (`SceneComponent.SetVisibility` _scannerlight false false)
        (`self.LightGreen`)
        (`self.OpenDoor`)
        (`KismetSystemLibrary.Delay` 3.0)))))

(event `LightGreen`
  (`SceneComponent.SetVisibility` (`self.PointLight`) true false))

(event `self.Cube.OnComponentHit`
  (params (HitComponent :type "PrimitiveComponent Object Reference") (OtherActor :type "Actor Object Reference") (OtherComp :type "PrimitiveComponent Object Reference") (NormalImpulse :type "Vector Structure") (Hit :type "HitResult Structure (by ref)")))

(fn `UserConstructionScript`
  (`parent.UserConstructionScript`))