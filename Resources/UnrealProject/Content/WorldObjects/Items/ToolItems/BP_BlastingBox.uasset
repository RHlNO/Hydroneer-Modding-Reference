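; BP_BlastingBox is an explosive tool item that blasts holes in voxel terrain when mouse-activated.
; Activation starts its particle systems, waits briefly, spawns BP_Explosion, then destroys the box.
; A sphere overlap filtered to VoxelWorld carves terrain via RemoveSphere, with a failed-cast fallback to the game controller's relic plant dig check.
; Construction caches the HydronixController as CastleControl and disables auto-activation on the main particle system.
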(event `/Game/WorldObjects/Items/BP_ParentItem.OverrideMouseActivated`
  (params (Component :type "ActorComponent Object Reference"))
  (`ActorComponent.Activate` (`self.ParticleSystem`) false)
  (`ActorComponent.Activate` (`self.ParticleSystem4`) false)
  (`ActorComponent.Activate` (`self.ParticleSystem7`) false)
  (`ActorComponent.Activate` (`self.ParticleSystem3`) false)
  (`ActorComponent.Activate` (`self.ParticleSystem8`) false)
  (`ActorComponent.Activate` (`self.ParticleSystem6`) false)
  (`ActorComponent.Activate` (`self.ParticleSystem2`) false)
  (`ActorComponent.Activate` (`self.ParticleSystem1`) false)
  (`ActorComponent.Activate` (`self.ParticleSystem9`) false)
  (`ActorComponent.Activate` (`self.ParticleSystem10`) false)
  (`ActorComponent.Activate` (`self.ParticleSystem5`) false)
  (`KismetSystemLibrary.Delay` 2.0)
  (bind _returnvalue (`|SpawnActorFromClass` "/Game/WorldObjects/Particles/BP_Explosion.BP_Explosion_C" (`self.GetTransform`) "Undefined" "OverrideRootScale" null null))
  (`ActorComponent.Activate` (`/Game/WorldObjects/Particles/BP_Explosion.ParticleSystem` _returnvalue) false)
  (bind _outactors (`KismetSystemLibrary.SphereOverlapActors` (`self.K2_GetActorLocation`) 600.0 (`self.NewVar_0_0`) "/Voxel/VoxelWorld.VoxelWorld_C"))
  (for _array_element _outactors
    (bind _asvoxel_world (cast `VoxelWorld` _array_element)
      (:`then`
        (`VoxelSphereTools.RemoveSphere` _asvoxel_world (`self.K2_GetActorLocation`) 30.0 true true))
      (:`CastFailed`
        (`/Game/BP_GameController.DigCheckForRelicPlants` (cast `/Game/BP_GameController` (`GameplayStatics.GetPlayerController` 0) :!pure true) _array_element))))
  (`self.K2_DestroyActor`))

(fn `UserConstructionScript`
  (`parent.UserConstructionScript`)
  (bind _outactors (`GameplayStatics.GetAllActorsOfClass` "/Game/ModIndex/HydronixController.HydronixController_C"))
  (set `self.CastleControl` (`|GetArrayItem` _outactors))
  (`ActorComponent.SetAutoActivate` (`self.ParticleSystem`) false))