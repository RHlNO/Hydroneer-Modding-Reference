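; Creative-mode and cheat tool item that gives the local player world-editing hotkeys.
; BeginPlay creates the F7Menu cheat widget, which supplies settings and spawn selection, and a toggleable world map.
; Input events center the mouse and trace under it to spawn, clone, delete or rotate items.
; Timers feed water items and generate pan gems, while Tick applies vertical flight input and the time-of-day freeze.
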(event `InputAction|RotateZ`
  (params (Key :type "Key Structure"))
  (:`Pressed`
    (`self.CenterMouse`)
    (bind _asbp_parent_item (cast `/Game/WorldObjects/Items/BP_ParentItem` (`.HitActor` (`GameplayStatics.BreakHitResult` (`PlayerController.GetHitResultUnderCursorByChannel` (`GameplayStatics.GetPlayerController` 0) "TraceTypeQuery1" true)))))
    (`self.K2_AddActorLocalRotation` _asbp_parent_item (struct :`Yaw` 90.0) false false)))

(event `InputAction|RotateY`
  (params (Key :type "Key Structure"))
  (:`Pressed`
    (`self.CenterMouse`)
    (bind _asbp_parent_item (cast `/Game/WorldObjects/Items/BP_ParentItem` (`.HitActor` (`GameplayStatics.BreakHitResult` (`PlayerController.GetHitResultUnderCursorByChannel` (`GameplayStatics.GetPlayerController` 0) "TraceTypeQuery1" true)))))
    (`self.K2_AddActorLocalRotation` _asbp_parent_item (struct :`Pitch` 90.0) false false)))

(event `InputAction|RotateX`
  (params (Key :type "Key Structure"))
  (:`Pressed`
    (`self.CenterMouse`)
    (bind _asbp_parent_item (cast `/Game/WorldObjects/Items/BP_ParentItem` (`.HitActor` (`GameplayStatics.BreakHitResult` (`PlayerController.GetHitResultUnderCursorByChannel` (`GameplayStatics.GetPlayerController` 0) "TraceTypeQuery1" true)))))
    (`self.K2_AddActorLocalRotation` _asbp_parent_item (struct :`Roll` 90.0) false false)))

(event `Key|O`
  (params (Key :type "Key Structure"))
  (bind _cheatmenu (`self.CheatMenu`))
  ;[1 1 1] Creative Mode Key Binds
  (:`Pressed`
    (set `/Game/F7Menu/F7Menu.CategorySelect` (+ (`/Game/F7Menu/F7Menu.CategorySelect` _cheatmenu) 1) _cheatmenu)
    (`/Game/F7Menu/F7Menu.UpdateSpawnItems` _cheatmenu :!label _label)))

(event `Key|I`
  (params (Key :type "Key Structure"))
  (bind _cheatmenu (`self.CheatMenu`))
  ;[1 1 1] Creative Mode Key Binds
  (:`Pressed`
    (set `/Game/F7Menu/F7Menu.CategorySelect` (- (`/Game/F7Menu/F7Menu.CategorySelect` _cheatmenu) 1) _cheatmenu)
    (goto _label)))

(event `self.ReceiveBeginPlay`
  (bind _returnvalue (`GameplayStatics.GetPlayerController` 0))
  (`self.SetOwner` _returnvalue)
  (if (not (`KismetSystemLibrary.IsValid` (`self.CheatMenu`)))
    (`self.EnableInput` _returnvalue)
    (bind _returnvalue_2 (`|CreateWidget` "/Game/F7Menu/F7Menu.F7Menu_C" _returnvalue))
    (bind _output_get (set `self.CheatMenu` _returnvalue_2))
    (`UserWidget.AddToViewport` _output_get 0)
    (`Widget.SetVisibility` _output_get "Visible")
    (bind _returnvalue_3 (`|CreateWidget` "/Game/UI/UI_WorldMap.UI_WorldMap_C" _returnvalue))
    (bind _output_get_2 (set `self.WorldMap` _returnvalue_3))
    (`UserWidget.AddToViewport` _output_get_2 0)
    (`Widget.SetVisibility` _output_get_2 "Collapsed")
    (`/Game/F7Menu/F7Menu.LoadSavedInfo` (`self.CheatMenu`))))

(event `Key|L`
  (params (Key :type "Key Structure"))
  (bind _cheatmenu (`self.CheatMenu`))
  ;[1 1 1] Creative Mode Key Binds
  (:`Pressed`
    (set `/Game/F7Menu/F7Menu.ClassSelect` (+ (`/Game/F7Menu/F7Menu.ClassSelect` _cheatmenu) 1) _cheatmenu)
    (`/Game/F7Menu/F7Menu.UpdateSpawnItems` _cheatmenu :!label _label_2)))

(event `Key|K`
  (params (Key :type "Key Structure"))
  (bind _cheatmenu (`self.CheatMenu`))
  ;[1 1 1] Creative Mode Key Binds
  (:`Pressed`
    (set `/Game/F7Menu/F7Menu.ClassSelect` (- (`/Game/F7Menu/F7Menu.ClassSelect` _cheatmenu) 1) _cheatmenu)
    (goto _label_2)))

(event `InputAction|FlightToggle`
  (params (Key :type "Key Structure"))
  (bind _cheatmenu (`self.CheatMenu`))
  (bind _flightcheck (`/Game/F7Menu/F7Menu.FlightCheck` _cheatmenu))
  (:`Pressed`
    (`CheckBox.SetIsChecked` _flightcheck (not (`CheckBox.IsChecked` _flightcheck)))
    (`/Game/F7Menu/F7Menu.ToggleFlight` _cheatmenu false)))

(event `InputAction|CreateItem`
  (params (Key :type "Key Structure"))
  (bind _cheatmenu (`self.CheatMenu`))
  (bind (_bblockinghit _binitialoverlap _time _distance _location _impactpoint _normal _impactnormal _physmat _hitactor) (`GameplayStatics.BreakHitResult` (`PlayerController.GetHitResultUnderCursorByChannel` (`GameplayStatics.GetPlayerController` 0) "TraceTypeQuery1" true)))
  ;[1 1 1] Creative Mode Key Binds
  (:`Pressed`
    (if (`CheckBox.IsChecked` (`/Game/F7Menu/F7Menu.CreativeToggle` _cheatmenu))
      (`self.CenterMouse`)
      (bind _output (`/Game/F7Menu/F7Menu.UpdateSpawnItems` _cheatmenu))
      (bind _returnvalue (`|SpawnActorFromClass` _output (`KismetMathLibrary.MakeTransform` (`KismetMathLibrary.MakeVector` (.x _location) (.y _location) (+ (.z _location) 60.0))) "Undefined" "OverrideRootScale" null null))
      (bind _asbp_parent_item (cast `/Game/WorldObjects/Items/BP_ParentItem` _returnvalue))
      (set `/Game/WorldObjects/Items/BP_ParentItem.PaidFor?` true _asbp_parent_item)
      (set `/Game/WorldObjects/Items/BP_ParentItem.BeingCarried?` true _asbp_parent_item)
      (bind _asbp_parent_resource (cast `/Game/WorldObjects/Items/ResourceItems/BP_ParentResource` _returnvalue)
        (:`then`
          (set `/Game/WorldObjects/Items/ResourceItems/BP_ParentResource.Size` (`/Game/F7Menu/F7Menu.SpawnSize` (`self.CheatMenu`)) _asbp_parent_resource)
          (`self.OverrideLoaded` _asbp_parent_resource))
        (:`CastFailed`
          _))
      (`self.ItemDropped` _asbp_parent_item))))

(event `InputAction|CollisionToggle`
  (params (Key :type "Key Structure"))
  (bind _cheatmenu (`self.CheatMenu`))
  (bind _collisioncheck (`/Game/F7Menu/F7Menu.CollisionCheck` _cheatmenu))
  (:`Pressed`
    (`CheckBox.SetIsChecked` _collisioncheck (not (`CheckBox.IsChecked` _collisioncheck)))
    (`/Game/F7Menu/F7Menu.ToggleCollision` _cheatmenu false)))

(event `InputAction|DeleteItem`
  (params (Key :type "Key Structure"))
  (bind (_bblockinghit _binitialoverlap _time _distance _location _impactpoint _normal _impactnormal _physmat _hitactor) (`GameplayStatics.BreakHitResult` (`PlayerController.GetHitResultUnderCursorByChannel` (`GameplayStatics.GetPlayerController` 0) "TraceTypeQuery1" true)))
  ;[1 1 1] Creative Mode Key Binds
  (:`Pressed`
    (if (`CheckBox.IsChecked` (`/Game/F7Menu/F7Menu.CreativeToggle` (`self.CheatMenu`)))
      (`self.CenterMouse`)
      (bind _asbp_parent_item (cast `/Game/WorldObjects/Items/BP_ParentItem` _hitactor)
        (:`then`
          (cast `/Game/WorldObjects/Items/ToolItems/BP_WorldControl` _hitactor
            (:`CastFailed`
              (`self.K2_DestroyActor` _asbp_parent_item))))
        (:`CastFailed`
          (bind _asbp_parent_vehicle (cast `/Game/WorldObjects/Vehicles/BP_ParentVehicle` _hitactor))
          (`self.K2_DestroyActor` _asbp_parent_vehicle))))))

(event `Key|F7`
  (params (Key :type "Key Structure"))
  (bind _returnvalue (`GameplayStatics.GetPlayerController` 0))
  (bind _cheatmenu (`self.CheatMenu`))
  ;[1 1 1] Cheat Menu
  (:`Pressed`
    (switch `ESlateVisibility` (`/Game/F7Menu/F7Menu.MenuGlobalVis` _cheatmenu) :!label _label_3
      (:`Visible`
        (`/Game/F7Menu/F7Menu.ResetVis` _cheatmenu)
        (set `PlayerController.bShowMouseCursor` false _returnvalue))
      (:`Collapsed`
        (set `/Game/F7Menu/F7Menu.MenuGlobalVis` "Visible" _cheatmenu)
        (set `PlayerController.bShowMouseCursor` true (`GameplayStatics.GetPlayerController` 0))
        (`WidgetBlueprintLibrary.SetInputMode_GameAndUIEx` _returnvalue _cheatmenu)))))

(event `Key|Escape`
  (params (Key :type "Key Structure"))
  ;[1 1 1] Cheat Menu
  (:`Pressed`
    (goto _label_3)))

(event `InputAction|WaterSpawn`
  (params (Key :type "Key Structure"))
  (:`Pressed`
    (`self.CenterMouse`)
    (bind _output_get (set `self.A Pipe` (`.HitActor` (`GameplayStatics.BreakHitResult` (`PlayerController.GetHitResultUnderCursorByChannel` (`GameplayStatics.GetPlayerController` 0) "TraceTypeQuery1" true)))))
    (cast `/Game/WorldObjects/Items/BuildItems/BP_ParentWaterItem` _output_get
      (:`then`
        (bind _returnvalue (`KismetSystemLibrary.K2_SetTimerDelegate` (delegate `CustomEvent_1`) 1.0 true)))
      (:`CastFailed`
        (`KismetSystemLibrary.K2_ClearAndInvalidateTimerHandle` _returnvalue)))))

(event `Key|F3`
  (params (Key :type "Key Structure"))
  ;[1 1 1] GemsInPan
  (:`Pressed`
    (bind _newparam1 (`/Game/F7Menu/F7Menu.GetClosestObject` (`self.CheatMenu`) "/Game/WorldObjects/Items/ToolItems/BP_Pan.BP_Pan_C"))
    (bind _asbp_pan (cast `/Game/WorldObjects/Items/ToolItems/BP_Pan` _newparam1))
    (bind _returnvalue (`KismetSystemLibrary.K2_SetTimerDelegate` (delegate `CustomEvent_0`) 0.01 true)))
  (:`Released`
    (`KismetSystemLibrary.K2_ClearAndInvalidateTimerHandle` _returnvalue)))

(event `CustomEvent_0`
  ;[1 1 1] GemsInPan
  (`/Game/WorldObjects/Items/ToolItems/BP_Pan.GenerateGems` (stale `Key|F3` _asbp_pan)))

(event `InputAction|OpenMap`
  (params (Key :type "Key Structure"))
  (bind _worldmap (`self.WorldMap`))
  ;[1 1 1] Map
  (:`Pressed`
    (if (`Widget.IsVisible` _worldmap)
      (`Widget.SetVisibility` _worldmap "Collapsed")
      (else
        (`Widget.SetVisibility` _worldmap "Visible")))))

(event `CustomEvent_1`
  (bind _asbp_parent_water_item (cast `/Game/WorldObjects/Items/BuildItems/BP_ParentWaterItem` (`self.A Pipe`)))
  (`/Game/WorldObjects/Items/BuildItems/BP_ParentWaterItem.WaterIn` _asbp_parent_water_item "Box2" 1 (`/Game/F7Menu/F7Menu.WaterPressure` (`self.CheatMenu`))))

(event `InputAction|PlayerUp`
  (params (Key :type "Key Structure"))
  ;[1 1 1] Flight
  (:`Pressed`
    (set `self.ShiftHeld?` true))
  (:`Released`
    (set `self.ShiftHeld?` false)
    (`KismetSystemLibrary.Delay` 0.1 :!label _label_4)
    (set `MovementComponent.Velocity` (0.0 0.0 0.0) (`Character.CharacterMovement` (`GameplayStatics.GetPlayerCharacter` 0)) :!label _label_5)))

(event `InputAction|PlayerStop`
  (params (Key :type "Key Structure"))
  ;[1 1 1] Flight
  (:`Pressed`
    (goto _label_5)))

(event `InputAction|PlayerDown`
  (params (Key :type "Key Structure"))
  ;[1 1 1] Flight
  (:`Pressed`
    (set `self.CtrlHeld?` true))
  (:`Released`
    (set `self.CtrlHeld?` false)
    (goto _label_4)))

(event `InputAction|CloneItem`
  (params (Key :type "Key Structure"))
  (bind _returnvalue (`GameplayStatics.GetPlayerController` 0))
  (bind (_returnvalue_x _returnvalue_y _returnvalue_z) (`KismetMathLibrary.BreakVector` (`self.K2_GetActorLocation` (`GameplayStatics.GetPlayerPawn` 0))))
  (bind (_bblockinghit _binitialoverlap _time _distance _location _impactpoint _normal _impactnormal _physmat _hitactor) (`GameplayStatics.BreakHitResult` (`PlayerController.GetHitResultUnderCursorByChannel` _returnvalue "TraceTypeQuery1" true)))
  ;[1 1 1] Duplicate Items
  (:`Pressed`
    (if (`CheckBox.IsChecked` (`/Game/F7Menu/F7Menu.CreativeToggle` (`self.CheatMenu`)))
      (`self.CenterMouse`)
      (cast `/Game/WorldObjects/Items/ToolItems/BP_WorldControl` _hitactor
        (:`CastFailed`
          (cast `/Game/WorldObjects/Items/BP_ParentItem` _hitactor)
          (bind _asbp_parent_resource (cast `/Game/WorldObjects/Items/ResourceItems/BP_ParentResource` _hitactor)
            (:`then`
              _)
            (:`CastFailed`
              _))
          (bind _returnvalue_2 (`|SpawnActorFromClass` (`GameplayStatics.GetObjectClass` _hitactor) (`KismetMathLibrary.MakeTransform` (`KismetMathLibrary.MakeVector` (+ (/ (- (.x _location) _returnvalue_x) 2.0) _returnvalue_x) (+ (/ (- (.y _location) _returnvalue_y) 2.0) _returnvalue_y) (+ (/ (- (.z _location) _returnvalue_z) 2.0) _returnvalue_z))) "AdjustIfPossibleButAlwaysSpawn" "OverrideRootScale" _returnvalue null))
          (bind _asbp_parent_item (cast `/Game/WorldObjects/Items/BP_ParentItem` _returnvalue_2))
          (set `/Game/WorldObjects/Items/BP_ParentItem.PaidFor?` true _asbp_parent_item)
          (set `/Game/WorldObjects/Items/BP_ParentItem.BeingCarried?` false _asbp_parent_item)
          (bind _asbp_parent_resource_2 (cast `/Game/WorldObjects/Items/ResourceItems/BP_ParentResource` _returnvalue_2))
          (set `/Game/WorldObjects/Items/ResourceItems/BP_ParentResource.Size` (`/Game/WorldObjects/Items/ResourceItems/BP_ParentResource.Size` _asbp_parent_resource) _asbp_parent_resource_2)
          (`self.OverrideLoaded` _asbp_parent_resource_2))))))

(event `self.ReceiveTick`
  (params (DeltaSeconds :type "Float (single-precision)"))
  (bind _returnvalue (`GameplayStatics.GetPlayerPawn` 0))
  (bind _cheatmenu (`self.CheatMenu`))
  (bind _maxacceleration (`CharacterMovementComponent.MaxAcceleration` (`Character.CharacterMovement` (`GameplayStatics.GetPlayerCharacter` 0))))
  (`|ExecutionSequence`
    (:`then_0`
      ;[1 1 1] Flight
      (if (`self.ShiftHeld?`)
        (`Pawn.AddMovementInput` _returnvalue (`KismetMathLibrary.MakeVector` 0.0 0.0 _maxacceleration) 100.0 false)
        (elif (`self.CtrlHeld?`)
          (`Pawn.AddMovementInput` _returnvalue (`KismetMathLibrary.MakeVector` 0.0 0.0 (* _maxacceleration -1.0)) 100.0 false))))
    (:`then_1`
      ;[1 1 1] Time Freeze
      (if (`CheckBox.IsChecked` (`/Game/F7Menu/F7Menu.TimeFreeze` _cheatmenu))
        (set `/Game/WorldObjects/BP_DayNightCycle.Hour` (`/Game/F7Menu/F7Menu.Hour` _cheatmenu) (`/Game/F7Menu/F7Menu.DayNight` _cheatmenu))))))

(fn `CenterMouse`
  (bind (_returnvalue_x _returnvalue_y) (`KismetMathLibrary.BreakVector2D` (`WidgetLayoutLibrary.GetViewportSize`)))
  (`PlayerController.SetMouseLocation` (`GameplayStatics.GetPlayerController` 0) (`KismetMathLibrary.FTrunc` (/ _returnvalue_x 2.0)) (`KismetMathLibrary.FTrunc` (/ _returnvalue_y 2.0))))

(fn `UserConstructionScript`
  (`parent.UserConstructionScript`))