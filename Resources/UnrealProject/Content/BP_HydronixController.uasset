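; Hydronix controller, a child class that varies the player's startup based on the game instance's LoadDone flag.
; On first load, BeginPlay runs the parent startup and sets the flag.
; When already set, it skips the parent, frees the player and character, creates the HUD with a movement mode and spawns BP_StoreBookcase.
; Tick, highlighting and crosshair tracing only call the parent; the HUD variable assignment is unconnected.
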(event `self.ReceiveBeginPlay`
  (bind _output_get (set `self.GameInstance` (cast `/Game/BP_GameInstance` (`GameplayStatics.GetGameInstance`) :!pure true)))
  (if (`/Game/BP_GameInstance.LoadDone?` _output_get)
    (`self.FreePlayer`)
    (bind _returnvalue (`|CreateWidget` "/Game/UI/UI_HUD.UI_HUD_C"))
    (`UserWidget.AddToViewport` _returnvalue 0)
    (set `/Game/UI/UI_HUD.CurrentMovementMode` "NewEnumerator0" _returnvalue)
    (set `/Game/BP_GameCharacter.Free?` true (cast `/Game/BP_GameCharacter` (`GameplayStatics.GetPlayerCharacter` 0) :!pure true))
    (`|SpawnActorFromClass` "/Game/WorldObjects/StoreItems/BuildCosmetics/BP_StoreBookcase.BP_StoreBookcase_C" (`KismetMathLibrary.MakeTransform` (0.0 0.0 0.0)) "Undefined" "OverrideRootScale" null null)
    (else
      (`parent.ReceiveBeginPlay`)
      (set `/Game/BP_GameInstance.LoadDone?` true _output_get))))

(event `self.HighlightObject`
  (params (Actor :type "Actor Object Reference"))
  (`parent.HighlightObject` Actor))

(event `self.ReceiveTick`
  (params (DeltaSeconds :type "Float (single-precision)"))
  (`parent.ReceiveTick` DeltaSeconds))

(event `self.CrosshairTrace`
  (`parent.CrosshairTrace`))

(fn `UserConstructionScript`
  (`parent.UserConstructionScript`))